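; BPO_GR_InvenItemInfo is a UObject holding one inventory item instance: data table row, Guid, amount, actor, rotation and inventory references.
; Setters fill it directly, from an item info struct, or from loot info with a new Guid, and CreateStruct converts it back to a struct.
; Clone constructs a copy with a fresh Guid, while helpers toggle rotation and flag an empty amount.
; The struct conversions omit the owner inventory reference.
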(fn SetAllMembers
  (params (InDataTableHndle :type Data%20Table%20Row%20Handle%20Structure) (InGuid :type Guid%20Structure) (InAmount :type Integer) (InActor :type Actor%20Object%20Reference) (InRotated :type Boolean) (InInventoryRef :type BPO%20GR%20Inventory%20Object%20Reference) (InOwnerInventoryRef :type BPO%20GR%20Inventory%20Object%20Reference))
  (Variables|Default|SetDataTableHandle InDataTableHndle)
  (Variables|Default|SetGuid InGuid)
  (Variables|Default|SetAmount InAmount)
  (Variables|Default|SetActor InActor)
  (Variables|Default|SetRotated InRotated)
  (Variables|Default|SetInventoryRef InInventoryRef)
  (Variables|Default|SetOwnerInventoryRef InOwnerInventoryRef))

(fn SetMembers
  (params (InDataTableHndle :type Data%20Table%20Row%20Handle%20Structure) (InGuid :type Guid%20Structure) (InAmount :type Integer) (InActor :type Actor%20Object%20Reference))
  (Variables|Default|SetDataTableHandle InDataTableHndle)
  (Variables|Default|SetGuid InGuid)
  (Variables|Default|SetAmount InAmount)
  (Variables|Default|SetActor InActor))

(fn EmptyAmount
  (return (<= (Variables|Default|GetAmount) 0)))

(fn Rotate
  (Variables|Default|SetRotated (not (Variables|Default|GetRotated))))

(fn Clone
  (bind _returnvalue (Game|ConstructObjectfromClass "BPO_GR_InvenItemInfo_C"))
  (bind _output_get (LocalVariables|SetLocalClone _returnvalue))
  (CallFunction|SetAllMembers _output_get (Variables|Default|GetDataTableHandle) (Guid|NewGuid) (Variables|Default|GetAmount) (Variables|Default|GetActor) (Variables|Default|GetRotated) (Variables|Default|GetInventoryRef) (Variables|Default|GetOwnerInventoryRef))
  (return (LocalVariables|GetLocalClone)))

(fn CreateStruct
  (return (Utilities|Struct|MakeS_GR_InvenItemInfo (Variables|Default|GetDataTableHandle) (Variables|Default|GetGuid) "(ChunkIndex_42_CD2BF50345BF9A1FA956AA835E3DADBA=0,SlotIndex_29_277281E743D41F5A7B4963B58ABB6819=0,ContainerRef_45_1F083FA4414BFF09D19137B94E3BDE4D=None)" (Variables|Default|GetAmount) (Variables|Default|GetActor) (Variables|Default|GetRotated) (Variables|Default|GetInventoryRef))))

(fn SetMembersfromStruct
  (params (InInvenItemInfo :type S%20GR%20Inven%20Item%20Info%20Structure))
  (bind (_tablerowhandle _guid _slotid _amount _actor _rotated _inventoryref) (Utilities|Struct|BreakS_GR_InvenItemInfo InInvenItemInfo))
  (CallFunction|SetAllMembers _tablerowhandle _guid _amount _actor _rotated _inventoryref))

(fn SetMembersbyLootInfo
  (params (InLootItemInfo :type S%20GR%20Loot%20Item%20Info%20Structure))
  (bind (_datatablehandle _amount) (Utilities|Struct|BreakS_GR_LootItemInfo InLootItemInfo))
  (Variables|Default|SetDataTableHandle _datatablehandle)
  (Variables|Default|SetAmount _amount)
  (Variables|Default|SetGuid (Guid|NewGuid)))