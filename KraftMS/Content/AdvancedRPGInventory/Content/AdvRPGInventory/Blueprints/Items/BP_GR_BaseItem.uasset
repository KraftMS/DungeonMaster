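; BP_GR_BaseItem is the base world item actor for the RPG inventory, supporting interaction and dropping.
; BeginPlay constructs its item-info object, filling it from the data table handle, amount and a new GUID unless the inventory created the item.
; Drop enables physics; Tick keeps the widget above the simulating mesh and stops simulation once it rests, after a short delay.
; Interact actions come from item data; outlines use overlay materials on pickup and equip meshes.
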(event Custom|Drop
  (bind _staticmesh_pickup (Variables|Default|GetStaticMesh_Pickup))
  (Utilities|IsValid (Variables|/Script/Engine.StaticMeshComponent|GetStaticMesh (Variables|Default|GetStaticMesh_Pickup))
    (:Is%20Valid
      (Collision|SetCollisionEnabled _staticmesh_pickup "QueryAndPhysics")
      (Physics|SetSimulatePhysics _staticmesh_pickup true)
      (Variables|Default|SetCheckStop false)
      (Utilities|FlowControl|Delay 0.2)
      (Variables|Default|SetCheckStop true))))

(event EventBeginPlay
  (bind _returnvalue (Game|ConstructObjectfromClass "/Game/AdvRPGInventory/Blueprints/UObjects/BPO_GR_InvenItemInfo.BPO_GR_InvenItemInfo_C"))
  (Variables|Default|SetInvenItemInfoRef _returnvalue)
  (if (not (Variables|Default|GetCreated%20from%20inventory))
    (Default|SetMembers (Variables|Default|GetInvenItemInfoRef) (Variables|Editable|GetItemDataHandle) (Guid|NewGuid) (Variables|Editable|GetItemAmount) self)))

(event Collision|EventActorBeginOverlap
  (params (OtherActor :type Actor%20Object%20Reference)))

(event EventTick
  (params (DeltaSeconds :type Float%20%28single-precision%29))
  (bind _staticmesh_pickup (Variables|Default|GetStaticMesh_Pickup))
  (bind _staticmesh_pickup_2 (Variables|Default|GetStaticMesh_Pickup))
  (Utilities|FlowControl|Sequence
    (:then_0
      (Utilities|IsValid (Variables|/Script/Engine.StaticMeshComponent|GetStaticMesh _staticmesh_pickup_2)
        (:Is%20Valid
          (if (Class|SceneComponent|IsAnySimulatingPhysics _staticmesh_pickup_2)
            (Transformation|SetWorldLocationAndRotation (Variables|Default|GetWidget) (+ (Transformation|GetWorldLocation _staticmesh_pickup_2) "0.000000,0.000000,42.000000") "0, 0, 0" false false)
            (if (Variables|Default|GetCheckStop)
              (if (Math|Vector|VectorIsZero (Transformation|GetComponentVelocity _staticmesh_pickup))
                (Physics|SetSimulatePhysics _staticmesh_pickup false)))))))))

(fn ConstructionScript)

(fn CanInteract
  (return true))

(fn GetInteractActions
  (bind (_found _returnvalue) (CallFunction|FindItemData (Variables|Default|GetInvenItemInfoRef)))
  (if _found
    (return (.InteractActions (Utilities|Struct|BreakS_GR_ItemTableData _returnvalue)))))

(fn ShowOutline
  (params (InVisible :type Boolean))
  (bind _staticmesh_pickup (Variables|Default|GetStaticMesh_Pickup))
  (bind _skeletalmesh_equip (Variables|Default|GetSkeletalMesh_Equip))
  (Utilities|FlowControl|Sequence
    (:then_0
      (Utilities|IsValid (Variables|/Script/Engine.StaticMeshComponent|GetStaticMesh (Variables|Default|GetStaticMesh_Pickup))
        (:Is%20Valid
          (if InVisible
            (Rendering|Material|SetOverlayMaterial _staticmesh_pickup "/Game/AdvRPGInventory/Demo/Materials/M_GI_Outline_Inst.M_GI_Outline_Inst" :!class /Script/Engine.MeshComponent)
            (else
              (Rendering|Material|SetOverlayMaterial _staticmesh_pickup 0 :!class /Script/Engine.MeshComponent))))))
    (:then_1
      (Utilities|IsValid (Variables|/Script/Engine.SkeletalMeshComponent|GetSkeletalMeshAsset (Variables|Default|GetSkeletalMesh_Equip))
        (:Is%20Valid
          (if InVisible
            (Rendering|Material|SetOverlayMaterial _skeletalmesh_equip "/Game/AdvRPGInventory/Demo/Materials/M_GI_Outline_Inst.M_GI_Outline_Inst" :!class /Script/Engine.MeshComponent)
            (else
              (Rendering|Material|SetOverlayMaterial _skeletalmesh_equip 0 :!class /Script/Engine.MeshComponent))))))
    (:then_2
      (return true))))