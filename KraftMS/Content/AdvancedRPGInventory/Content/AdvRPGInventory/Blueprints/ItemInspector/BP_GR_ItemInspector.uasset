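; BP_GR_ItemInspector is an inventory item inspector actor built around a SceneCaptureComponent2D.
; BeginPlay restricts the capture's show-only list to the actor itself.
; Start looks up and stores item data.
; Its logic to set a skeletal or static capture mesh, enable per-frame capture and return the render target is disconnected, so it never runs.
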(event EventBeginPlay
  (Utilities|Array|Clear (Variables|/Script/Engine.SceneCaptureComponent|GetShowOnlyActors (Variables|Default|GetSceneCaptureComponent2D)))
  (Utilities|Array|Add (Variables|/Script/Engine.SceneCaptureComponent|GetShowOnlyActors (Variables|Default|GetSceneCaptureComponent2D)) self))

(event Collision|EventActorBeginOverlap
  (params (OtherActor :type Actor%20Object%20Reference)))

(event EventTick
  (params (DeltaSeconds :type Float%20%28single-precision%29)))

(fn ConstructionScript)

(fn Start
  (params (InInvenItemInfoRef :type BPO%20GR%20Inven%20Item%20Info%20Object%20Reference%20%28by%20ref%29))
  (bind (_found _returnvalue) (CallFunction|FindItemData InInvenItemInfoRef))
  (if _found
    (bind _output_get (LocalVariables|SetLocalItemData _returnvalue))))