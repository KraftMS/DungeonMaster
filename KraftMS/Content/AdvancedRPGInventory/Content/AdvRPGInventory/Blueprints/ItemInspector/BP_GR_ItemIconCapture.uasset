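; Actor that renders inventory item icons with a SceneCapture2D that has the actor itself on its show-only list.
; GetCaptureIconTexture, for items flagged for captured icons, creates a render target sized by slot footprint and caches it by item GUID, releasing it on forced re-creation.
; UpdateScene is called before each capture but does nothing, as its logic for rebuilding the skeletal mesh with static-mesh attachments is disconnected.
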(event EventBeginPlay
  (Utilities|Array|Add (Variables|/Script/Engine.SceneCaptureComponent|GetShowOnlyActors (Variables|Default|GetSceneCaptureComponent2D)) self))

(fn ConstructionScript)

(fn GetCaptureIconTexture
  (params (InInvenItemInfo :type S%20GR%20Inven%20Item%20Info%20Structure) (InReCreate :type Boolean))
  (bind _icontexture (Variables|Default|GetIconTexture))
  (bind _icontexture_2 (Variables|Default|GetIconTexture))
  (bind _scenecapturecomponent2d (Variables|Default|GetSceneCaptureComponent2D))
  (bind _guid (Utilities|Struct|BreakS_GR_InvenItemInfo InInvenItemInfo))
  (bind _guid_2 (Utilities|Struct|BreakS_GR_InvenItemInfo InInvenItemInfo))
  (bind (_value _returnvalue) (Utilities|Map|Find _icontexture _guid))
  (bind (_value_2 _returnvalue_2) (Utilities|Map|Find _icontexture_2 _guid_2))
  (bind _returnvalue_3 (CallFunction|FindItemDatabyTableRow (Utilities|Struct|BreakS_GR_InvenItemInfo InInvenItemInfo)))
  (bind _output_get (LocalVariables|SetLocalItemData _returnvalue_3))
  (if (.UseCaptureItemIcon (Utilities|Struct|BreakS_GR_ItemTableData _output_get))
    (if InReCreate
      (if _returnvalue_2
        (Class|KismetRenderingLibrary|ReleaseRenderTarget2D _value_2)
        (Utilities|Map|Remove (Variables|Default|GetIconTexture) (Utilities|Struct|BreakS_GR_InvenItemInfo InInvenItemInfo)))
      (elif _returnvalue
        (return _value)
        (else
          _)))
    (CallFunction|UpdateScene InInvenItemInfo)
    (bind _returnvalue_4 (Rendering|CreateRenderTarget2D (* (.SlotWidth (Utilities|Struct|BreakS_GR_ItemTableData (LocalVariables|GetLocalItemData))) 90) (* (.SlotHeight (Utilities|Struct|BreakS_GR_ItemTableData (LocalVariables|GetLocalItemData))) 90) "RTF_RGBA16f"))
    (bind _output_get_2 (LocalVariables|SetLocalRenderTarget _returnvalue_4))
    (Variables|/Script/Engine.SceneCaptureComponent2D|SetTextureTarget _scenecapturecomponent2d _output_get_2)
    (Rendering|SceneCapture|CaptureScene _scenecapturecomponent2d :!class /Script/Engine.SceneCaptureComponent2D)
    (Variables|/Script/Engine.SceneCaptureComponent2D|SetTextureTarget (Variables|Default|GetSceneCaptureComponent2D) 0)
    (Utilities|Map|Add (Variables|Default|GetIconTexture) (Utilities|Struct|BreakS_GR_InvenItemInfo InInvenItemInfo) (LocalVariables|GetLocalRenderTarget))
    (return (LocalVariables|GetLocalRenderTarget))))

(fn UpdateScene
  (params (InItemInfo :type S%20GR%20Inven%20Item%20Info%20Structure%20%28by%20ref%29)))