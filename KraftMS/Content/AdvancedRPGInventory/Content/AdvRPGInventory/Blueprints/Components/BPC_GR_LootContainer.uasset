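; Actor component that makes its owner a lootable container, moving its items into the player's BPC_GR_AdvInventoryComp.
; Opening reuses or creates one loot bar widget, rebinds its buttons and switches input to UI-friendly mode.
; Slots are built from DataTable rows; taken entries become new inventory item objects with fresh GUIDs.
; Take All, or taking the last item, closes the window and destroys the owning actor.
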(fn OpenLootWidget
  (params (InPlayerActor :type Actor%20Object%20Reference))
  (bind _returnvalue (Game|GetPlayerController 0))
  (bind _returnvalue_2 (Game|GetPlayerController 0))
  (Variables|Default|SetOpenPlayerActor InPlayerActor)
  (bind _foundwidgets (Widget|GetAllWidgetsOfClass "/Game/AdvRPGInventory/Blueprints/Widgets/Widget_RPG_LootBarWindow.Widget_RPG_LootBarWindow_C" true))
  (bind _output_get (LocalVariables|SetLocalWidgetArray _foundwidgets))
  (if (Utilities|Array|IsEmpty _output_get)
    (bind _returnvalue_3 (UserInterface|CreateWidget "/Game/AdvRPGInventory/Blueprints/Widgets/Widget_RPG_LootBarWindow.Widget_RPG_LootBarWindow_C"))
    (Variables|Default|SetLootBarHUD _returnvalue_3)
    (UserInterface|Viewport|AddtoViewport (Variables|Default|GetLootBarHUD) 0)
    (else
      (bind _output_get_2 (Variables|Default|SetLootBarHUD (Utilities|Array|Get(acopy) _output_get)))
      (Widget|SetVisibility _output_get_2 "Visible")))
  (Utilities|FlowControl|Sequence
    (:then_0
      (CallFunction|UpdateWidgets))
    (:then_1
      (EventDispatchers|UnbindallEventsfromOnClickButtonTake (Variables|/Game/AdvRPGInventory/Blueprints/Widgets/Widget_RPG_LootBarWindow.Widget_RPG_LootBarWindow_C|GetWidget_RPG_LootBar (Variables|Default|GetLootBarHUD)))
      (EventDispatchers|UnbindallEventsfromOnClickButtonTakeAll (Variables|/Game/AdvRPGInventory/Blueprints/Widgets/Widget_RPG_LootBarWindow.Widget_RPG_LootBarWindow_C|GetWidget_RPG_LootBar (Variables|Default|GetLootBarHUD)))
      (EventDispatchers|UnbindallEventsfromOnClickButtonClose (Variables|/Game/AdvRPGInventory/Blueprints/Widgets/Widget_RPG_LootBarWindow.Widget_RPG_LootBarWindow_C|GetWidget_RPG_LootBar (Variables|Default|GetLootBarHUD)))
      (EventDispatchers|BindEventtoOnClickButtonTakeAll (Variables|/Game/AdvRPGInventory/Blueprints/Widgets/Widget_RPG_LootBarWindow.Widget_RPG_LootBarWindow_C|GetWidget_RPG_LootBar (Variables|Default|GetLootBarHUD)) (EventDispatchers|CreateEvent :!event OnClickButtonTakeAll))
      (EventDispatchers|BindEventtoOnClickButtonClose (Variables|/Game/AdvRPGInventory/Blueprints/Widgets/Widget_RPG_LootBarWindow.Widget_RPG_LootBarWindow_C|GetWidget_RPG_LootBar (Variables|Default|GetLootBarHUD)) (EventDispatchers|CreateEvent :!event OnClickButtonClose)))
    (:then_2
      (Variables|/Script/Engine.PlayerController|SetbShowMouseCursor _returnvalue_2 true)
      (Input|SetInputModeGameandUI _returnvalue_2 (Variables|Default|GetLootBarHUD) "DoNotLock" false false)
      (Input|SetIgnoreLookInput _returnvalue true)
      (Input|SetIgnoreMoveInput _returnvalue true))))

(fn UpdateWidgets
  (Widget|Panel|ClearChildren (Variables|/Game/AdvRPGInventory/Blueprints/Widgets/Widget_RPG_LootBar.Widget_RPG_LootBar_C|GetVerticalBox (Variables|/Game/AdvRPGInventory/Blueprints/Widgets/Widget_RPG_LootBarWindow.Widget_RPG_LootBarWindow_C|GetWidget_RPG_LootBar (Variables|Default|GetLootBarHUD))))
  (for (_array_element _array_index) (Variables|Editable|GetLootItemInfoArray)
    (bind _output_get (LocalVariables|SetLocalLootItemInfo _array_element))
    (LocalVariables|SetLocalItemIndex _array_index)
    (bind _returnvalue (Utilities|GetDataTableRow (.DataTable (Utilities|Struct|BreakDataTableRowHandle (.DataTableHandle (Utilities|Struct|BreakS_GR_LootItemInfo _output_get)))) (.RowName (Utilities|Struct|BreakDataTableRowHandle (.DataTableHandle (Utilities|Struct|BreakS_GR_LootItemInfo _output_get)))))
      (:then
        (LocalVariables|SetLocalItemData _returnvalue)
        (bind _returnvalue_2 (UserInterface|CreateWidget "/Game/AdvRPGInventory/Blueprints/Widgets/Widget_RPG_LootBarSlot.Widget_RPG_LootBarSlot_C"))
        (bind _output_get_2 (LocalVariables|SetLocalLootBarSlot _returnvalue_2))
        (Class|VerticalBox|AddChildtoVerticalBox (Variables|/Game/AdvRPGInventory/Blueprints/Widgets/Widget_RPG_LootBar.Widget_RPG_LootBar_C|GetVerticalBox (Variables|/Game/AdvRPGInventory/Blueprints/Widgets/Widget_RPG_LootBarWindow.Widget_RPG_LootBarWindow_C|GetWidget_RPG_LootBar (Variables|Default|GetLootBarHUD))) _output_get_2)
        (Default|UpdateWidget (LocalVariables|GetLocalLootBarSlot) (.InventoryIcon (Utilities|Struct|BreakS_GR_ItemTableData (LocalVariables|GetLocalItemData))) (Utilities|Struct|BreakS_GR_LootItemInfo (LocalVariables|GetLocalLootItemInfo)) (.Name (Utilities|Struct|BreakS_GR_ItemTableData (LocalVariables|GetLocalItemData))))
        (Variables|/Game/AdvRPGInventory/Blueprints/Widgets/Widget_RPG_LootBarSlot.Widget_RPG_LootBarSlot_C|SetItemIndex (LocalVariables|GetLocalLootBarSlot) (LocalVariables|GetLocalItemIndex))
        (EventDispatchers|BindEventtoOnClickButtonLootBarSlot (LocalVariables|GetLocalLootBarSlot) (EventDispatchers|CreateEvent :!event OnClickButtonLootSlot))))))

(fn CloseLootBarWidget
  (bind _returnvalue (Game|GetPlayerController 0))
  (bind _returnvalue_2 (Game|GetPlayerController 0))
  (Utilities|IsValid (Variables|Default|GetLootBarHUD)
    (:Is%20Valid
      (Widget|SetVisibility (Variables|Default|GetLootBarHUD) "Hidden")
      (Variables|/Script/Engine.PlayerController|SetbShowMouseCursor _returnvalue false)
      (Input|SetInputModeGameOnly _returnvalue false)
      (Input|SetIgnoreLookInput _returnvalue_2 false)
      (Input|SetIgnoreMoveInput _returnvalue_2 false))))

(fn CanOpenLootBar
  (if (> (Utilities|Array|Length (Variables|Editable|GetLootItemInfoArray)) 0)
    (return true)))

(fn OnClickButtonLootSlot
  (params (InItemIndex :type Integer))
  (bind _returniteminfo (CallFunction|CreateInvenItemInfo (Utilities|Array|Get(acopy) (Variables|Editable|GetLootItemInfoArray) InItemIndex)))
  (bind _returnvalue (Default|AddItemtoPlayerInventory (Actor|GetComponentbyClass (Game|GetPlayerCharacter 0) "/Game/AdvRPGInventory/Blueprints/Components/BPC_GR_AdvInventoryComp.BPC_GR_AdvInventoryComp_C") _returniteminfo))
  (if _returnvalue
    (Utilities|Array|RemoveIndex (Variables|Editable|GetLootItemInfoArray) InItemIndex)
    (CallFunction|UpdateWidgets)
    (Audio|PlaySound2D "/Game/AdvRPGInventory/Demo/Audio/SFX/MS_UI_Hover.MS_UI_Hover" 1.0 1.0 0.0 0 0)
    (if (Utilities|Array|IsEmpty (Variables|Editable|GetLootItemInfoArray))
      (CallFunction|CloseLootBarWidget)
      (Actor|DestroyActor (Components|GetOwner)))))

(fn OnClickButtonTakeAll
  (bind _returniteminfo (CallFunction|CreateInvenItemInfoArray (Variables|Editable|GetLootItemInfoArray)))
  (Default|AddItemArraytoPlayerInventory (Actor|GetComponentbyClass (Game|GetPlayerCharacter 0) "/Game/AdvRPGInventory/Blueprints/Components/BPC_GR_AdvInventoryComp.BPC_GR_AdvInventoryComp_C") _returniteminfo)
  (Utilities|Array|Clear (Variables|Editable|GetLootItemInfoArray))
  (CallFunction|UpdateWidgets)
  (Audio|PlaySound2D "/Game/AdvRPGInventory/Demo/Audio/SFX/MS_UI_Select.MS_UI_Select" 1.0 1.0 0.0 0 0)
  (CallFunction|CloseLootBarWidget)
  (Actor|DestroyActor (Components|GetOwner)))

(fn OnClickButtonClose
  (CallFunction|CloseLootBarWidget)
  (Audio|PlaySound2D "/Game/AdvRPGInventory/Demo/Audio/SFX/MS_UI_Select.MS_UI_Select" 1.0 1.0 0.0 0 0))

(fn CreateInvenItemInfo
  (params (InLootItemInfo :type S%20GR%20Loot%20Item%20Info%20Structure%20%28by%20ref%29))
  (bind (_datatablehandle _amount) (Utilities|Struct|BreakS_GR_LootItemInfo InLootItemInfo))
  (bind _returnvalue (Game|ConstructObjectfromClass "/Game/AdvRPGInventory/Blueprints/UObjects/BPO_GR_InvenItemInfo.BPO_GR_InvenItemInfo_C"))
  (bind _output_get (LocalVariables|SetLocalItemInfo _returnvalue))
  (Default|SetMembers _output_get _datatablehandle (Guid|NewGuid) _amount)
  (return (LocalVariables|GetLocalItemInfo)))

(fn CreateInvenItemInfoArray
  (params (InLootItemInfoArray :type Array%20of%20S%20GR%20Loot%20Item%20Info%20Structures))
  (for _array_element InLootItemInfoArray
    (bind _returniteminfo (CallFunction|CreateInvenItemInfo _array_element))
    (Utilities|Array|Add (LocalVariables|GetLocalItemInfoArray) _returniteminfo))
  (return (LocalVariables|GetLocalItemInfoArray)))