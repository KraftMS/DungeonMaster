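; Quickbar container component that binds inventory items to numbered quick slots for an RPG inventory.
; Slots store only item GUIDs, resolved through the owner inventory to fill widget icons and amounts or to clear missing items.
; Binding requires AllowQuickSlotBind; manual binding moves an item from its previous slot, while auto-binding takes the first empty slot without a duplicate check.
; Loading saved slots re-points their container reference to this component.
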(event Custom|Init
  (params (InOwnerInventoryRef :type BPO%20GR%20Inventory%20Object%20Reference) (InQuickSlotCount :type Integer))
  (Variables|Default|SetOwnerInventoryRef InOwnerInventoryRef)
  (Utilities|Array|Clear (Variables|Default|GetQuickSlotInfoArray))
  (for _index (range 0 (- InQuickSlotCount 1))
    (Utilities|Array|Add (Variables|Default|GetQuickSlotInfoArray) (Utilities|Struct|MakeS_GR_QuickSlotInfo _index self (Utilities|Struct|MakeGuid)))))

(event EventBeginPlay)

(fn InitWidgets
  (params (InContainerWidget :type User%20Widget%20Object%20Reference) (In%20Quick%20Slot%20Widgets :type Array%20of%20User%20Widget%20Object%20References))
  (Variables|Default|SetContainerWidget InContainerWidget)
  (LocalVariables|SetLocalSlotWidgets In%20Quick%20Slot%20Widgets)
  (Utilities|Array|Clear (Variables|Default|GetQuick%20Slot%20Widgets))
  (for (_array_element _array_index) (LocalVariables|GetLocalSlotWidgets)
    (bind _aswidget_gr_quick_slot (Utilities|Casting|CastToWidget_GR_QuickSlot _array_element))
    (bind _output_get (LocalVariables|SetLocalQuickSlot _aswidget_gr_quick_slot))
    (bind _output_get_2 (Variables|/Game/AdvRPGInventory/Demo/Blueprints/Widgets/Slots/Widget_GR_QuickSlot.Widget_GR_QuickSlot_C|SetSlotIndex _output_get _array_index))
    (Default|UpdateQuickSlotKey (LocalVariables|GetLocalQuickSlot) true (+ _output_get_2 1))
    (Variables|/Game/AdvRPGInventory/Demo/Blueprints/Widgets/Slots/Widget_GR_QuickSlot.Widget_GR_QuickSlot_C|SetContainerComp (LocalVariables|GetLocalQuickSlot) self)
    (Utilities|Array|Add (Variables|Default|GetQuick%20Slot%20Widgets) (LocalVariables|GetLocalQuickSlot)))
  (CallFunction|UpdateWidgets))

(fn TryBindSlot
  (params (InBindSlotIndex :type Integer) (InBindInvenItemInfoRef :type BPO%20GR%20Inven%20Item%20Info%20Object%20Reference))
  (bind _returnvalue (CallFunction|FindItemData InBindInvenItemInfoRef))
  (bind _output_get (LocalVariables|SetLocalBindItemData _returnvalue))
  (if (.AllowQuickSlotBind (Utilities|Struct|BreakS_GR_ItemTableData _output_get))
    (bind (_returnvalue_2 _returnslotindex) (CallFunction|FindSameSlot InBindInvenItemInfoRef))
    (if _returnvalue_2
      (bind _output_get_2 (LocalVariables|SetLocalFindSameSlotIndex _returnslotindex))
      (CallFunction|ClearSlot _output_get_2))
    (Utilities|Struct|SetmembersinS_GR_QuickSlotInfo (Utilities|Array|Get(acopy) (Variables|Default|GetQuickSlotInfoArray) InBindSlotIndex) (Variables|/Game/AdvRPGInventory/Blueprints/UObjects/BPO_GR_InvenItemInfo.BPO_GR_InvenItemInfo_C|GetGuid InBindInvenItemInfoRef) "(ChunkIndex_42_CD2BF50345BF9A1FA956AA835E3DADBA=0,SlotIndex_29_277281E743D41F5A7B4963B58ABB6819=0,InvenItemInfoRef_49_DEBB75A94A0ECC66AF0E1AA70A676C8E=None,ContainerRef_45_BFEDBCC64FC12F95768818A6D7059A5E=None,SlotType_33_BB3856664944119713AD97B51651B24F=NewEnumerator0,EquipmentType_35_D197B73E4845E573079D4A9B62665DF1=NewEnumerator13,AttachmentType_38_E3A2D4F14280B1399589FB8510B158DE=NewEnumerator0)" "(TableRowHandle_108_95EE096842DE52AA04A2D1B7B6405EB8=(DataTable=None,RowName=\"\"),Guid_90_59F74E2847898EA9A61D8FB6F5B3634A=00000000000000000000000000000000,SlotID_112_827A30634B2B8718940D67B2F7FF335C=(ChunkIndex_42_CD2BF50345BF9A1FA956AA835E3DADBA=0,SlotIndex_29_277281E743D41F5A7B4963B58ABB6819=0,ContainerRef_45_1F083FA4414BFF09D19137B94E3BDE4D=None),Amount_5_62DB2267439500D86A52E0B2266494D2=1,Actor_71_FCD35A0D415FF7A362349EA94EE99155=None,Rotated_18_66B00C8648A7E3BEB56C4282929D015D=False,InventoryRef_111_86F4AEE1471C73D11DE4ED842BA86B4B=None)")))

(fn FindSameSlot
  (params (InInvenItemInfoRef :type BPO%20GR%20Inven%20Item%20Info%20Object%20Reference))
  (for (_array_element _array_index) (Variables|Default|GetQuickSlotInfoArray)
    (LocalVariables|SetLocalIndex _array_index)
    (if (== (Utilities|Struct|BreakS_GR_QuickSlotInfo _array_element) (Variables|/Game/AdvRPGInventory/Blueprints/UObjects/BPO_GR_InvenItemInfo.BPO_GR_InvenItemInfo_C|GetGuid InInvenItemInfoRef))
      (return true (LocalVariables|GetLocalIndex))))
  (return false -1))

(fn ClearSlot
  (params (InSlotIndex :type Integer))
  (if (Utilities|Array|IsValidIndex (Variables|Default|GetQuickSlotInfoArray) InSlotIndex)
    (Utilities|Struct|SetmembersinS_GR_QuickSlotInfo (Utilities|Array|Get(acopy) (Variables|Default|GetQuickSlotInfoArray) InSlotIndex) (Utilities|Struct|MakeGuid))))

(fn IsEmptySlot
  (params (InSlotIndex :type Integer))
  (return (not (Guid|IsValidGuid (Utilities|Struct|BreakS_GR_QuickSlotInfo (Utilities|Array|Get(acopy) (Variables|Default|GetQuickSlotInfoArray) InSlotIndex))))))

(fn UpdateWidgets
  (for (_array_element _array_index) (Variables|Default|GetQuick%20Slot%20Widgets)
    (LocalVariables|SetLocalWidget _array_element)
    (LocalVariables|SetLocalIndex _array_index)
    (bind (_found _returniteminforef) (Default|FindItemInfobyGuid (Variables|Default|GetOwnerInventoryRef) (Utilities|Struct|BreakS_GR_QuickSlotInfo (Utilities|Array|Get(acopy) (Variables|Default|GetQuickSlotInfoArray) (LocalVariables|GetLocalIndex)))))
    (if _found
      (bind _output_get (LocalVariables|SetLocalItemInfoRef _returniteminforef))
      (bind (_found_2 _returnvalue) (CallFunction|FindItemData _output_get))
      (if _found_2
        (Default|UpdateWidget (LocalVariables|GetLocalWidget) true (.QuickSlotIcon (Utilities|Struct|BreakS_GR_ItemTableData _returnvalue)) (.AllowStacking (Utilities|Struct|BreakS_GR_ItemTableData _returnvalue)) (Variables|/Game/AdvRPGInventory/Blueprints/UObjects/BPO_GR_InvenItemInfo.BPO_GR_InvenItemInfo_C|GetAmount (LocalVariables|GetLocalItemInfoRef)))
        (else
          (Default|UpdateWidget (LocalVariables|GetLocalWidget) false 0 false :!label _label)))
      (else
        (goto _label)))))

(fn RefreshSlots)

(fn LoadfromSaveInfoQuickbarContainer
  (params (InQuickSlotInfoArray :type Array%20of%20S%20GR%20Quick%20Slot%20Info%20Structures))
  (bind _output_get (Variables|Default|SetQuickSlotInfoArray InQuickSlotInfoArray))
  (for _index (range 0 (- (Utilities|Array|Length _output_get) 1))
    (Utilities|Struct|SetmembersinS_GR_QuickSlotInfo (Utilities|Array|Get(acopy) (Variables|Default|GetQuickSlotInfoArray) _index) self)))

(fn UpdateSlots
  (for _index (range 0 (- (Utilities|Array|Length (Variables|Default|GetQuickSlotInfoArray)) 1))
    (bind _output_get (LocalVariables|SetLocalSlotIndex _index))
    (if (Guid|IsValidGuid (Utilities|Struct|BreakS_GR_QuickSlotInfo (Utilities|Array|Get(acopy) (Variables|Default|GetQuickSlotInfoArray) _output_get)))
      (bind _found (Default|FindItemInfobyGuid (Variables|Default|GetOwnerInventoryRef) (Utilities|Struct|BreakS_GR_QuickSlotInfo (Utilities|Array|Get(acopy) (Variables|Default|GetQuickSlotInfoArray) _output_get))))
      (if (not _found)
        (CallFunction|ClearSlot (LocalVariables|GetLocalSlotIndex))))))

(fn TryBindSlotAuto
  (params (InBindInvenItemInfoRef :type BPO%20GR%20Inven%20Item%20Info%20Object%20Reference))
  (Utilities|FlowControl|Sequence
    (:then_0
      (bind _returnvalue (CallFunction|FindItemData InBindInvenItemInfoRef))
      (bind _output_get (LocalVariables|SetLocalBindItemData _returnvalue))
      (if (.AllowQuickSlotBind (Utilities|Struct|BreakS_GR_ItemTableData _output_get))
        (bind (_returnvalue_2 _returnslotindex) (CallFunction|FindEmptySlot))
        (if _returnvalue_2
          (Utilities|Struct|SetmembersinS_GR_QuickSlotInfo (Utilities|Array|Get(acopy) (Variables|Default|GetQuickSlotInfoArray) _returnslotindex) (Variables|/Game/AdvRPGInventory/Blueprints/UObjects/BPO_GR_InvenItemInfo.BPO_GR_InvenItemInfo_C|GetGuid InBindInvenItemInfoRef))
          (return true))))
    (:then_1
      (return false))))

(fn FindEmptySlot
  (for (_array_element _array_index) (Variables|Default|GetQuickSlotInfoArray)
    (LocalVariables|SetLocalIndex _array_index)
    (if (not (Guid|IsValidGuid (Utilities|Struct|BreakS_GR_QuickSlotInfo _array_element)))
      (return true (LocalVariables|GetLocalIndex))))
  (return false -1))

(fn GetSlot
  (params (InIndex :type Integer))
  (return (Utilities|Array|Get(acopy) (Variables|Default|GetQuickSlotInfoArray) InIndex)))