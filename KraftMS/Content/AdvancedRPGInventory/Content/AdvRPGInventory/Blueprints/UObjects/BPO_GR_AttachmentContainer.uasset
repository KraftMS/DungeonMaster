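; Inventory container object that holds an owning item's attachments in slots typed by attachment type, built on a base container class.
; Placement succeeds only in an empty slot of matching type; moves clear the source slot, and auto-move takes the first fit.
; Slot widgets refresh with each item's icon and name, plus ammo count for magazine attachments via the owner inventory.
; TryAddItem, ContainsActor and the mag-slot ammo search are unwired stubs, and CanAddAmmo always returns false.
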(fn UpdateWidgetsBase
  (Utilities|FlowControl|Sequence
    (:then_0
      (for _index (range 0 (- (Utilities|Array|Length (Variables|Default|GetWidgetSlotChunkInfoArray)) 1))
        (bind _output_get (LocalVariables|SetLocalChunkIndex _index))
        (for _array_element (Utilities|Struct|BreakS_GR_WidgetSlotChunkInfo (Utilities|Array|Get(acopy) (Variables|Default|GetWidgetSlotChunkInfoArray) _output_get))
          (Class|BPIGRSlotWidgetInterface|UpdateWidgetAttachmentSlot(Message) _array_element false))))
    (:then_1
      (bind _returnvaluearray (CallFunction|GetAllItemsBase))
      (for _array_element_2 _returnvaluearray
        (bind _output_get_2 (LocalVariables|SetLocalItemInfoRef _array_element_2))
        (bind (_found _returnvalue) (Default|FindItemDataFl (Variables|Default|GetOwnerInventory) _output_get_2))
        (if _found
          (LocalVariables|SetLocalItemData _returnvalue)
          (Utilities|FlowControl|Sequence
            (:then_0
              (if (Utilities|Enum|Equal(Enum) (.AttachmentType (Utilities|Struct|BreakS_GR_ItemTableData (LocalVariables|GetLocalItemData))) "NewEnumerator5")
                (bind (_returnvalue_2 _ammo _maxammo) (CallFunction|GetMagItemAmmoCount))
                (LocalVariables|SetLocalAmountText (Utilities|Text|FormatText "{0}/{1}" _ammo _maxammo))))
            (:then_1
              (bind _returnslotinfo (CallFunction|FindSlotInfobyItemInfoBase (LocalVariables|GetLocalItemInfoRef)))
              (Class|BPIGRSlotWidgetInterface|UpdateWidgetAttachmentSlot(Message) (CallFunction|GetInvenSlotWidgetbyIndexBase (.ChunkIndex (Utilities|Struct|BreakS_GR_InvenSlotInfo _returnslotinfo)) (.SlotIndex (Utilities|Struct|BreakS_GR_InvenSlotInfo _returnslotinfo))) true (.InventoryIcon (Utilities|Struct|BreakS_GR_ItemTableData (LocalVariables|GetLocalItemData))) (.Name (Utilities|Struct|BreakS_GR_ItemTableData (LocalVariables|GetLocalItemData))) (LocalVariables|GetLocalAmountText)))))))))

(fn TryMoveItemBase
  (params (InMoveItemInfoRef :type BPO%20GR%20Inven%20Item%20Info%20Object%20Reference) (InFromSlotInfo :type S%20GR%20Inven%20Slot%20Info%20Structure) (InToSlotInfo :type S%20GR%20Inven%20Slot%20Info%20Structure))
  (LocalVariables|SetLocalFromSlotInfo InFromSlotInfo)
  (bind _result (CallFunction|TryPlaceItemBase InMoveItemInfoRef InToSlotInfo (LocalVariables|GetLocalFromSlotInfo)))
  (if _result
    (Default|ClearItemInfoBase (Utilities|Struct|BreakS_GR_InvenSlotInfo (LocalVariables|GetLocalFromSlotInfo)) (LocalVariables|GetLocalFromSlotInfo))
    (return true "")
    (else
      (return false ""))))

(fn TryMoveItemAutoBase
  (params (InMoveItemInfoRef :type BPO%20GR%20Inven%20Item%20Info%20Object%20Reference) (InFromSlotInfo :type S%20GR%20Inven%20Slot%20Info%20Structure))
  (for _index (range 0 (- (Utilities|Array|Length (Variables|Default|GetSlotChunkInfoArray)) 1))
    (LocalVariables|SetLocalChunkIndex _index)
    (for _index_2 (range 0 (- (Utilities|Array|Length (Utilities|Struct|BreakS_GR_SlotChunkInfo (Utilities|Array|Get(acopy) (Variables|Default|GetSlotChunkInfoArray) (LocalVariables|GetLocalChunkIndex)))) 1))
      (LocalVariables|SetLocalSlotIndex _index_2)
      (LocalVariables|SetLocalToSlotInfo (CallFunction|GetSlotInfobyIndexBase (LocalVariables|GetLocalChunkIndex) (LocalVariables|GetLocalSlotIndex)))
      (bind _result (CallFunction|TryPlaceItemBase InMoveItemInfoRef (LocalVariables|GetLocalToSlotInfo) InFromSlotInfo))
      (if _result
        (Default|ClearItemInfoBase (Utilities|Struct|BreakS_GR_InvenSlotInfo InFromSlotInfo) InFromSlotInfo)
        (return true (LocalVariables|GetLocalToSlotInfo) ""))))
  (return false "" ""))

(fn LoadfromSaveInfoBase
  (params (InOwnerItemGuid :type Guid%20Structure) (InOwnerItemActor :type Actor%20Object%20Reference) (InSlotChunkInfoArray :type Array%20of%20S%20GR%20Slot%20Chunk%20Info%20Structures) (InItemInfoArray :type Array%20of%20S%20GR%20Inven%20Item%20Info%20Structures))
  (|CallParentFunction InOwnerItemGuid InOwnerItemActor InSlotChunkInfoArray InItemInfoArray)
  (return))

(fn TryPlaceItemBase
  (params (InPlaceInvenItemInfoRef :type BPO%20GR%20Inven%20Item%20Info%20Object%20Reference) (InToSlotInfo :type S%20GR%20Inven%20Slot%20Info%20Structure) (InFromSlotInfo :type S%20GR%20Inven%20Slot%20Info%20Structure))
  (bind (_chunkindex _slotindex) (Utilities|Struct|BreakS_GR_InvenSlotInfo InToSlotInfo))
  (if (CallFunction|CanMoveItem :InToChunkIndex _chunkindex :InToSlotIndex _slotindex :InPlaceItemInfoRef InPlaceInvenItemInfoRef)
    (CallFunction|SetItemInfoBase InToSlotInfo InPlaceInvenItemInfoRef)
    (return true "")))

(fn FindEmptySlotIndexfromType
  (params (InAttachmentType :type E_GR_InvenAttachmentType%20Enum :default "NewEnumerator0"))
  (for _index (range 0 (- (Utilities|Array|Length (Variables|Default|GetSlotChunkInfoArray)) 1))
    (LocalVariables|SetLocalChunkIndex _index)
    (for (_array_element _array_index) (Utilities|Struct|BreakS_GR_SlotChunkInfo (Utilities|Array|Get(acopy) (Variables|Default|GetSlotChunkInfoArray) (LocalVariables|GetLocalChunkIndex)))
      (LocalVariables|SetLocalSlotInfo _array_element)
      (LocalVariables|SetLocalSlotIndex _array_index)
      (if (and (Utilities|Enum|Equal(Enum) (Utilities|Struct|BreakS_GR_InvenSlotInfo (LocalVariables|GetLocalSlotInfo)) InAttachmentType) (not (Utilities|IsValid (Utilities|Struct|BreakS_GR_InvenSlotInfo (LocalVariables|GetLocalSlotInfo)))))
        (return true (LocalVariables|GetLocalChunkIndex) (LocalVariables|GetLocalSlotIndex)))))
  (return false -1 -1))

(fn TryAddItem
  (params (InInvenItemInfoRef :type BPO%20GR%20Inven%20Item%20Info%20Object%20Reference)))

(fn CanMoveItem
  (params (InToChunkIndex :type Integer) (InToSlotIndex :type Integer) (InPlaceItemInfo :type S%20GR%20Inven%20Item%20Info%20Structure%20%28by%20ref%29) (InPlaceItemInfoRef :type BPO%20GR%20Inven%20Item%20Info%20Object%20Reference))
  (bind _returnvalue (Default|FindItemDataFl (Variables|Default|GetOwnerInventory) InPlaceItemInfoRef))
  (return (and (Utilities|Enum|Equal(Enum) (.AttachmentType (Utilities|Struct|BreakS_GR_ItemTableData _returnvalue)) (Utilities|Struct|BreakS_GR_InvenSlotInfo (Utilities|Array|Get(acopy) (Utilities|Struct|BreakS_GR_SlotChunkInfo (Utilities|Array|Get(acopy) (Variables|Default|GetSlotChunkInfoArray) InToChunkIndex)) InToSlotIndex))) (CallFunction|IsEmptySlotBase InToChunkIndex InToSlotIndex))))

(fn CanMoveItemAuto
  (params (InMoveItemInfo :type S%20GR%20Inven%20Item%20Info%20Structure) (InMoveItemInfoRef :type BPO%20GR%20Inven%20Item%20Info%20Object%20Reference))
  (for _index (range 0 (- (Utilities|Array|Length (Variables|Default|GetSlotChunkInfoArray)) 1))
    (LocalVariables|SetLocalChunkIndex _index)
    (for _index_2 (range 0 (- (Utilities|Array|Length (Utilities|Struct|BreakS_GR_SlotChunkInfo (Utilities|Array|Get(acopy) (Variables|Default|GetSlotChunkInfoArray) (LocalVariables|GetLocalChunkIndex)))) 1))
      (LocalVariables|SetLocalSlotIndex _index_2)
      (if (CallFunction|CanMoveItem (LocalVariables|GetLocalChunkIndex) (LocalVariables|GetLocalSlotIndex) InMoveItemInfo)
        (return true))))
  (return false))

(fn FindItemInfobyType
  (params (InAttachmentType :type E_GR_InvenAttachmentType%20Enum :default "NewEnumerator0"))
  (bind _returnvaluearray (CallFunction|GetAllItemsBase))
  (for _array_element _returnvaluearray
    (bind _output_get (LocalVariables|SetLocalItemInfoRef _array_element))
    (bind _returnvalue (Default|FindItemDataFl (Variables|Default|GetOwnerInventory) _output_get))
    (if (Utilities|Enum|Equal(Enum) (Utilities|Struct|BreakS_GR_ItemTableData _returnvalue) InAttachmentType)
      (return true "" (LocalVariables|GetLocalItemInfoRef))))
  (return false "" 0))

(fn CanAddAmmo
  (Utilities|FlowControl|Sequence
    (:then_1
      (return false))))

(fn ContainsActor
  (params (InActor :type Actor%20Object%20Reference)))

(fn FindMagAmmoSlotInfoCanAddAmmo)

(fn GetMagItemAmmoCount
  (Utilities|FlowControl|Sequence
    (:then_0
      (bind (_find _returniteminfo _returniteminforef) (CallFunction|FindItemInfobyType "NewEnumerator5"))
      (if _find
        (bind (_returnvalue _ammo _maxammo) (Default|GetMagItemAmmoCountFl :self (Variables|Default|GetOwnerInventory) :InMagItemInfoRef _returniteminforef))
        (return _returnvalue _ammo _maxammo)))
    (:then_1
      (return false 0 0))))

(fn InitFunc
  (params (InContainerName :type Name) (InOwnerItemGuid :type Guid%20Structure) (InOwnerItemActor :type Actor%20Object%20Reference) (InSlotInfoArray :type Array%20of%20S%20GR%20Inven%20Slot%20Info%20Structures))
  (Variables|Default|SetContainerName InContainerName)
  (Variables|Default|SetOwnerItemGuid InOwnerItemGuid)
  (Variables|Default|SetOwnerActor InOwnerItemActor)
  (Utilities|Array|Clear (Variables|Default|GetSlotChunkInfoArray))
  (Utilities|Struct|SetmembersinS_GR_SlotChunkInfo (LocalVariables|GetLocalEmptySlotChunkInfo) InSlotInfoArray)
  (Utilities|Array|Add (Variables|Default|GetSlotChunkInfoArray) (LocalVariables|GetLocalEmptySlotChunkInfo))
  (CallFunction|ResetSlotChunkInfoArrayBase))

(fn InitWidgetsBase
  (params (InputContainerWidget :type User%20Widget%20Object%20Reference) (InWidgetSlotChunkInfoArray :type Array%20of%20S%20GR%20Widget%20Slot%20Chunk%20Info%20Structures))
  (|CallParentFunction InputContainerWidget InWidgetSlotChunkInfoArray)
  (return))

(fn TryAddItemBase
  (params (InInvenItemInfoRef :type BPO%20GR%20Inven%20Item%20Info%20Object%20Reference) (InFromSlotInfo :type S%20GR%20Inven%20Slot%20Info%20Structure))
  (bind _returnvalue (|CallParentFunction InInvenItemInfoRef InFromSlotInfo))
  (return _returnvalue))