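; Inventory container object for equipment slots, where each slot accepts only items whose data lists its equipment type.
; Overrides base-container operations: add fills the first empty matching slot, place and move validate type, and swap finds the occupant by type.
; Changes fire an item-change call, and widget refresh redraws icon, name and, for two slot types, ammo counts.
; Item-to-slot lookup returns the first type-compatible slot without comparing item references.
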(fn UpdateWidgetsBase
  (Utilities|FlowControl|Sequence
    (:then_0
      (for _index (range 0 (- (Utilities|Array|Length (Variables|Default|GetWidgetSlotChunkInfoArray)) 1))
        (bind _output_get (LocalVariables|SetLocalChunkIndex _index))
        (for _array_element (Utilities|Struct|BreakS_GR_WidgetSlotChunkInfo (Utilities|Array|Get(acopy) (Variables|Default|GetWidgetSlotChunkInfoArray) _output_get))
          (Class|BPIGRSlotWidgetInterface|UpdateWidgetEquipSlot(Message) _array_element false))))
    (:then_1
      (bind _returnvaluearray (CallFunction|GetAllItemsBase))
      (for _array_element_2 _returnvaluearray
        (CallFunction|UpdateWidgetbyItemInfoBase false _array_element_2)))))

(fn TryMoveItemBase
  (params (InMoveItemInfoRef :type BPO%20GR%20Inven%20Item%20Info%20Object%20Reference) (InFromSlotInfo :type S%20GR%20Inven%20Slot%20Info%20Structure) (InToSlotInfo :type S%20GR%20Inven%20Slot%20Info%20Structure))
  (LocalVariables|SetLocalFromSlotInfo InFromSlotInfo)
  (bind (_result _returnplaceiteminfo) (CallFunction|TryPlaceItemBase InMoveItemInfoRef InToSlotInfo (LocalVariables|GetLocalFromSlotInfo)))
  (if _result
    (LocalVariables|SetLocalPlaceLootItemInfo _returnplaceiteminfo)
    (Default|ClearItemInfoBase (Utilities|Struct|BreakS_GR_InvenSlotInfo (LocalVariables|GetLocalFromSlotInfo)) (LocalVariables|GetLocalFromSlotInfo))
    (return true (LocalVariables|GetLocalPlaceLootItemInfo))))

(fn TryPlaceItemBase
  (params (InPlaceInvenItemInfoRef :type BPO%20GR%20Inven%20Item%20Info%20Object%20Reference) (InToSlotInfo :type S%20GR%20Inven%20Slot%20Info%20Structure) (InFromSlotInfo :type S%20GR%20Inven%20Slot%20Info%20Structure))
  (LocalVariables|SetLocalToSlotInfo InToSlotInfo)
  (if (CallFunction|CanPlaceItemBase InPlaceInvenItemInfoRef InFromSlotInfo InToSlotInfo)
    (Utilities|FlowControl|Sequence
      (:then_0
        (CallFunction|SetItemInfoBase InToSlotInfo InPlaceInvenItemInfoRef)
        (Default|CallOnChangeItemInfo))
      (:then_1
        (return true (Utilities|Struct|MakeS_GR_LootItemInfo (Variables|/Game/AdvRPGInventory/Blueprints/UObjects/BPO_GR_InvenItemInfo.BPO_GR_InvenItemInfo_C|GetDataTableHandle InPlaceInvenItemInfoRef) (Variables|/Game/AdvRPGInventory/Blueprints/UObjects/BPO_GR_InvenItemInfo.BPO_GR_InvenItemInfo_C|GetAmount InPlaceInvenItemInfoRef)))))))

(fn UpdateAllSlotInfobyItemInfoBase
  (|CallParentFunction))

(fn TryAddItemBase
  (params (InInvenItemInfoRef :type BPO%20GR%20Inven%20Item%20Info%20Object%20Reference) (InFromSlotInfo :type S%20GR%20Inven%20Slot%20Info%20Structure))
  (Utilities|FlowControl|Sequence
    (:then_0
      (bind (_found _returnvalue) (Default|FindItemDataFl (Variables|Default|GetOwnerInventory) InInvenItemInfoRef))
      (if _found
        (bind _output_get (LocalVariables|SetLocalItemData _returnvalue))
        (for _array_element (.EquipmentSlots (Utilities|Struct|BreakS_GR_ItemTableData _output_get))
          (bind _output_get_2 (LocalVariables|SetLocalEquipmentType _array_element))
          (bind (_find _returnslotid) (CallFunction|FindEmptyEquipSlotID _output_get_2))
          (if _find
            (bind _output_get_3 (LocalVariables|SetLocalToSlotID _returnslotid))
            (bind _returnslotinfo (Default|GetSlotInfobySlotIDFl (Variables|Default|GetOwnerInventory) _output_get_3))
            (CallFunction|SetItemInfoBase _returnslotinfo InInvenItemInfoRef)
            (Default|CallOnChangeItemInfo)
            (return true)))))
    (:then_1
      (return false))))

(fn CanPlaceItemBase
  (params (InMoveItemInfoRef :type BPO%20GR%20Inven%20Item%20Info%20Object%20Reference) (InFromSlotInfo :type S%20GR%20Inven%20Slot%20Info%20Structure) (InToSlotInfo :type S%20GR%20Inven%20Slot%20Info%20Structure) (InBlockSlotIndexArray :type Array%20of%20Integers) (InIgnoreItemRefArray :type Array%20of%20BPO%20GR%20Inven%20Item%20Info%20Object%20References))
  (bind _returnvalue (Default|FindItemDataFl (Variables|Default|GetOwnerInventory) InMoveItemInfoRef))
  (return (and (Utilities|Array|ContainsItem (.EquipmentSlots (Utilities|Struct|BreakS_GR_ItemTableData _returnvalue)) (Utilities|Struct|BreakS_GR_InvenSlotInfo InToSlotInfo)) true)))

(fn InitWidgetsBase
  (params (InputContainerWidget :type User%20Widget%20Object%20Reference) (InWidgetSlotChunkInfoArray :type Array%20of%20S%20GR%20Widget%20Slot%20Chunk%20Info%20Structures))
  (|CallParentFunction InputContainerWidget InWidgetSlotChunkInfoArray)
  (return))

(fn FindEmptyEquipSlotID
  (params (InEquipmentType :type E_GR_InvenEquipmentType%20Enum :default "NewEnumerator13"))
  (for _index (range 0 (- (Utilities|Array|Length (Variables|Default|GetSlotChunkInfoArray)) 1))
    (LocalVariables|SetLocalChunkIndex _index)
    (for (_array_element _array_index) (Utilities|Struct|BreakS_GR_SlotChunkInfo (Utilities|Array|Get(acopy) (Variables|Default|GetSlotChunkInfoArray) (LocalVariables|GetLocalChunkIndex)))
      (LocalVariables|SetLocalSlotInfo _array_element)
      (LocalVariables|SetLocalSlotIndex _array_index)
      (if (and (Utilities|Enum|Equal(Enum) (Utilities|Struct|BreakS_GR_InvenSlotInfo (LocalVariables|GetLocalSlotInfo)) InEquipmentType) (not (Utilities|IsValid (Utilities|Struct|BreakS_GR_InvenSlotInfo (LocalVariables|GetLocalSlotInfo)))))
        (return true (Utilities|Struct|MakeS_GR_InvenSlotID (LocalVariables|GetLocalChunkIndex) (LocalVariables|GetLocalSlotIndex) self)))))
  (return false ""))

(fn FindItemInfofromEquipType
  (params (InEquipType :type E_GR_InvenEquipmentType%20Enum :default "NewEnumerator13"))
  (for _array_element (Variables|Default|GetSlotChunkInfoArray)
    (for _array_element_2 (Utilities|Struct|BreakS_GR_SlotChunkInfo _array_element)
      (Utilities|IsValid (.InvenItemInfoRef (Utilities|Struct|BreakS_GR_InvenSlotInfo _array_element_2))
        (:Is%20Valid
          (LocalVariables|SetLocalItemInfoRef (.InvenItemInfoRef (Utilities|Struct|BreakS_GR_InvenSlotInfo _array_element_2)))
          (if (Utilities|Enum|Equal(Enum) (.EquipmentType (Utilities|Struct|BreakS_GR_InvenSlotInfo _array_element_2)) InEquipType)
            (return true (LocalVariables|GetLocalItemInfoRef)))))))
  (return false 0))

(fn ContainsActor
  (params (InActor :type Actor%20Object%20Reference))
  (bind _returnvaluearray (CallFunction|GetAllItemsBase))
  (for _array_element _returnvaluearray
    (Utilities|IsValid (Variables|/Game/AdvRPGInventory/Blueprints/UObjects/BPO_GR_InvenItemInfo.BPO_GR_InvenItemInfo_C|GetActor _array_element)
      (:Is%20Valid
        (if (== (Variables|/Game/AdvRPGInventory/Blueprints/UObjects/BPO_GR_InvenItemInfo.BPO_GR_InvenItemInfo_C|GetActor _array_element) InActor)
          (return true)))))
  (return false))

(fn FindEmptySlotInfofromType
  (params (InEquipmentType :type E_GR_InvenEquipmentType%20Enum :default "NewEnumerator13"))
  (for _index (range 0 (- (Utilities|Array|Length (Variables|Default|GetSlotChunkInfoArray)) 1))
    (LocalVariables|SetLocalChunkIndex _index)
    (for (_array_element _array_index) (Utilities|Struct|BreakS_GR_SlotChunkInfo (Utilities|Array|Get(acopy) (Variables|Default|GetSlotChunkInfoArray) (LocalVariables|GetLocalChunkIndex)))
      (LocalVariables|SetLocalSlotInfo _array_element)
      (LocalVariables|SetLocalSlotIndex _array_index)
      (if (and (Utilities|Enum|Equal(Enum) (Utilities|Struct|BreakS_GR_InvenSlotInfo (LocalVariables|GetLocalSlotInfo)) InEquipmentType) (not (Utilities|IsValid (Utilities|Struct|BreakS_GR_InvenSlotInfo (LocalVariables|GetLocalSlotInfo)))))
        (return true (LocalVariables|GetLocalSlotInfo)))))
  (return false ""))

(fn ResetSlotChunkInfoArray
  (for _index (range 0 (- (Utilities|Array|Length (Variables|Default|GetSlotChunkInfoArray)) 1))
    (LocalVariables|SetLocalChunkIndex _index)
    (for _index_2 (range 0 (- (Utilities|Array|Length (Utilities|Struct|BreakS_GR_SlotChunkInfo (Utilities|Array|Get(acopy) (Variables|Default|GetSlotChunkInfoArray) (LocalVariables|GetLocalChunkIndex)))) 1))
      (LocalVariables|SetLocalSlotIndex _index_2)
      (Utilities|Struct|SetmembersinS_GR_InvenSlotInfo (Utilities|Array|Get(acopy) (Utilities|Struct|BreakS_GR_SlotChunkInfo (Utilities|Array|Get(acopy) (Variables|Default|GetSlotChunkInfoArray) (LocalVariables|GetLocalChunkIndex))) (LocalVariables|GetLocalSlotIndex)) (LocalVariables|GetLocalChunkIndex) (LocalVariables|GetLocalSlotIndex) 0 self "NewEnumerator1"))))

(fn InitFunc
  (params (InContainerName :type Name) (InOwnerItemGuid :type Guid%20Structure) (InOwnerItemActor :type Actor%20Object%20Reference) (InSlotInfoArray :type Array%20of%20S%20GR%20Inven%20Slot%20Info%20Structures))
  (Variables|Default|SetContainerName InContainerName)
  (Variables|Default|SetOwnerActor InOwnerItemActor)
  (Utilities|Array|Clear (Variables|Default|GetSlotChunkInfoArray))
  (Utilities|Struct|SetmembersinS_GR_SlotChunkInfo (LocalVariables|GetLocalEmptySlotChunkInfo) InSlotInfoArray)
  (Utilities|Array|Add (Variables|Default|GetSlotChunkInfoArray) (LocalVariables|GetLocalEmptySlotChunkInfo))
  (CallFunction|ResetSlotChunkInfoArrayBase))

(fn UpdateWidgetbyItemInfoBase
  (params (InReCreateIconTexture :type Boolean) (InInvenItemInfoRef :type BPO%20GR%20Inven%20Item%20Info%20Object%20Reference))
  (bind (_found _returnvalue) (Default|FindItemDataFl (Variables|Default|GetOwnerInventory) InInvenItemInfoRef))
  (if _found
    (LocalVariables|SetLocalItemData _returnvalue)
    (bind _returnvalue_2 (CallFunction|FindSlotInfofromItemInfo InInvenItemInfoRef))
    (LocalVariables|SetLocalSlotWidget (CallFunction|GetInvenSlotWidgetbyIndexBase (.ChunkIndex (Utilities|Struct|BreakS_GR_InvenSlotInfo _returnvalue_2)) (.SlotIndex (Utilities|Struct|BreakS_GR_InvenSlotInfo _returnvalue_2))))
    (LocalVariables|SetLocalAmountText (Utilities|Text|MakeLiteralText ""))
    (Utilities|FlowControl|Sequence
      (:then_0
        (if (or (Utilities|Array|ContainsItem (.EquipmentSlots (Utilities|Struct|BreakS_GR_ItemTableData (LocalVariables|GetLocalItemData))) "NewEnumerator9") (Utilities|Array|ContainsItem (.EquipmentSlots (Utilities|Struct|BreakS_GR_ItemTableData (LocalVariables|GetLocalItemData))) "NewEnumerator10"))
          (bind (_returnvalue_3 _ammo _maxammo) (Default|GetWeaponItemAmmoCountFl (Variables|Default|GetOwnerInventory) InInvenItemInfoRef))
          (LocalVariables|SetLocalAmountText (Utilities|Text|FormatText "{0}/{1}" _ammo _maxammo))))
      (:then_1
        (Class|BPIGRSlotWidgetInterface|UpdateWidgetEquipSlot(Message) (LocalVariables|GetLocalSlotWidget) true (.InventoryIcon (Utilities|Struct|BreakS_GR_ItemTableData (LocalVariables|GetLocalItemData))) (.Name (Utilities|Struct|BreakS_GR_ItemTableData (LocalVariables|GetLocalItemData))) (LocalVariables|GetLocalAmountText))))))

(fn ResetSlotChunkInfoArrayBase
  (for _index (range 0 (- (Utilities|Array|Length (Variables|Default|GetSlotChunkInfoArray)) 1))
    (LocalVariables|SetLocalChunkIndex _index)
    (for _index_2 (range 0 (- (Utilities|Array|Length (Utilities|Struct|BreakS_GR_SlotChunkInfo (Utilities|Array|Get(acopy) (Variables|Default|GetSlotChunkInfoArray) (LocalVariables|GetLocalChunkIndex)))) 1))
      (LocalVariables|SetLocalSlotIndex _index_2)
      (Utilities|Struct|SetmembersinS_GR_InvenSlotInfo (Utilities|Array|Get(acopy) (Utilities|Struct|BreakS_GR_SlotChunkInfo (Utilities|Array|Get(acopy) (Variables|Default|GetSlotChunkInfoArray) (LocalVariables|GetLocalChunkIndex))) (LocalVariables|GetLocalSlotIndex)) (LocalVariables|GetLocalChunkIndex) (LocalVariables|GetLocalSlotIndex) 0 self "NewEnumerator1"))))

(fn FindItemInfotoSwapBase
  (params (InMoveItemInfoRef :type BPO%20GR%20Inven%20Item%20Info%20Object%20Reference) (InFromSlotInfo :type S%20GR%20Inven%20Slot%20Info%20Structure) (InToSlotInfo :type S%20GR%20Inven%20Slot%20Info%20Structure))
  (Utilities|FlowControl|Sequence
    (:then_0
      (bind (_found _returniteminforef) (CallFunction|FindItemInfofromEquipType (Utilities|Struct|BreakS_GR_InvenSlotInfo InToSlotInfo)))
      (if _found
        (return true _returniteminforef)))
    (:then_1
      (return false 0))))

(fn FindSlotInfofromItemInfo
  (params (InInvenItemInfoRef :type BPO%20GR%20Inven%20Item%20Info%20Object%20Reference))
  (bind (_found _returnvalue) (Default|FindItemDataFl (Variables|Default|GetOwnerInventory) InInvenItemInfoRef))
  (if _found
    (LocalVariables|SetLocalEquipmentTypeArray (Utilities|Struct|BreakS_GR_ItemTableData _returnvalue))
    (for _index (range 0 (- (Utilities|Array|Length (Variables|Default|GetSlotChunkInfoArray)) 1))
      (LocalVariables|SetLocalChunkIndex _index)
      (for (_array_element _array_index) (Utilities|Struct|BreakS_GR_SlotChunkInfo (Utilities|Array|Get(acopy) (Variables|Default|GetSlotChunkInfoArray) (LocalVariables|GetLocalChunkIndex)))
        (LocalVariables|SetLocalSlotInfo _array_element)
        (LocalVariables|SetLocalSlotIndex _array_index)
        (if (Utilities|Array|ContainsItem (LocalVariables|GetLocalEquipmentTypeArray) (Utilities|Struct|BreakS_GR_InvenSlotInfo (LocalVariables|GetLocalSlotInfo)))
          (return true (LocalVariables|GetLocalSlotInfo)))))
    (return false "")))