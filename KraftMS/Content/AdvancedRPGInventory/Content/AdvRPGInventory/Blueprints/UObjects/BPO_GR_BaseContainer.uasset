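; Base UObject for inventory containers in the RPG inventory system, storing item info references in slots grouped into chunks.
; It provides shared lookup, removal, weight totals and stack merging, while add, move, place and widget updates are stubs, apparently for subclass overrides.
; Slots and their widgets are tagged with chunk/slot indices and the container reference.
; Helpers convert items to save structs and rebuild item objects from save or loot data.
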(fn InitBase
  (params (InContainerName :type Name) (InOwnerInventory :type BPO%20GR%20Inventory%20Object%20Reference) (InSlotChunkInfoArray :type Array%20of%20S%20GR%20Slot%20Chunk%20Info%20Structures))
  (Variables|Default|SetContainerName InContainerName)
  (Variables|Default|SetOwnerInventory InOwnerInventory)
  (Variables|Default|SetSlotChunkInfoArray InSlotChunkInfoArray)
  (Base|ResetSlotChunkInfoArrayBase))

(fn UpdateAllSlotInfobyItemInfoBase)

(fn TryRemoveItemBase
  (params (InItemInfoRef :type BPO%20GR%20Inven%20Item%20Info%20Object%20Reference))
  (for _array_element (Variables|Default|GetSlotChunkInfoArray)
    (for _array_element_2 (Utilities|Struct|BreakS_GR_SlotChunkInfo _array_element)
      (bind _output_get (LocalVariables|SetLocalSlotInfo _array_element_2))
      (Utilities|IsValid (Utilities|Struct|BreakS_GR_InvenSlotInfo _output_get)
        (:Is%20Valid
          (if (== (Utilities|Struct|BreakS_GR_InvenSlotInfo _output_get) InItemInfoRef)
            (Base|ClearItemInfoBase (LocalVariables|GetLocalSlotInfo))
            (Default|CallOnChangeItemInfo)
            (return true)))))))

(fn UpdateWidgetsBase)

(fn TryMoveItemBase
  (params (InMoveItemInfoRef :type BPO%20GR%20Inven%20Item%20Info%20Object%20Reference) (InFromSlotInfo :type S%20GR%20Inven%20Slot%20Info%20Structure) (InToSlotInfo :type S%20GR%20Inven%20Slot%20Info%20Structure))
  (return false ""))

(fn TryMoveItemAutoBase
  (params (InMoveItemInfoRef :type BPO%20GR%20Inven%20Item%20Info%20Object%20Reference) (InFromSlotInfo :type S%20GR%20Inven%20Slot%20Info%20Structure))
  (return false "" ""))

(fn ContainsItemBase
  (params (InCheckItemInfoRef :type BPO%20GR%20Inven%20Item%20Info%20Object%20Reference))
  (for _array_element (Variables|Default|GetSlotChunkInfoArray)
    (for _array_element_2 (Utilities|Struct|BreakS_GR_SlotChunkInfo _array_element)
      (Utilities|IsValid (Utilities|Struct|BreakS_GR_InvenSlotInfo _array_element_2)
        (:Is%20Valid
          (if (== (Utilities|Struct|BreakS_GR_InvenSlotInfo _array_element_2) InCheckItemInfoRef)
            (return true)))))
    (return false)))

(fn ContainsSlotBase
  (params (InCheckSlotInfo :type S%20GR%20Inven%20Slot%20Info%20Structure))
  (if (== (Utilities|Struct|BreakS_GR_InvenSlotInfo InCheckSlotInfo) self)
    (return true)))

(fn LoadfromSaveInfoBase
  (params (InOwnerItemGuid :type Guid%20Structure) (InOwnerItemActor :type Actor%20Object%20Reference) (InSlotChunkInfoArray :type Array%20of%20S%20GR%20Slot%20Chunk%20Info%20Structures) (InItemInfoArray :type Array%20of%20S%20GR%20Inven%20Item%20Info%20Structures)))

(fn GetSlotInfobyIndexBase
  (params (InChuckIndex :type Integer) (InSlotIndex :type Integer))
  (if (Utilities|Array|IsValidIndex (Variables|Default|GetSlotChunkInfoArray) InChuckIndex)
    (return (Utilities|Array|Get(acopy) (Utilities|Struct|BreakS_GR_SlotChunkInfo (Utilities|Array|Get(acopy) (Variables|Default|GetSlotChunkInfoArray) InChuckIndex)) InSlotIndex))))

(fn IsEmptySlotBase
  (params (InputChunkIndex :type Integer) (InputSlotIndex :type Integer))
  (Utilities|IsValid (Utilities|Struct|BreakS_GR_InvenSlotInfo (Utilities|Array|Get(acopy) (Utilities|Struct|BreakS_GR_SlotChunkInfo (Utilities|Array|Get(acopy) (Variables|Default|GetSlotChunkInfoArray) InputChunkIndex)) InputSlotIndex))
    (:Is%20Valid
      (return false))
    (:Is%20Not%20Valid
      (return true))))

(fn GetWeightBase
  (bind _returnvaluearray (Base|GetAllItemsBase))
  (for _array_element _returnvaluearray
    (LocalVariables|SetLocalAmount (Variables|/Game/AdvRPGInventory/Blueprints/UObjects/BPO_GR_InvenItemInfo.BPO_GR_InvenItemInfo_C|GetAmount _array_element))
    (bind _returnvalue (Default|FindItemDataFl (Variables|Default|GetOwnerInventory) _array_element))
    (LocalVariables|SetLocalWeight (+ (* (.Weight (Utilities|Struct|BreakS_GR_ItemTableData _returnvalue)) (LocalVariables|GetLocalAmount)) (LocalVariables|GetLocalWeight))))
  (return (LocalVariables|GetLocalWeight)))

(fn TryAddItemBase
  (params (InInvenItemInfoRef :type BPO%20GR%20Inven%20Item%20Info%20Object%20Reference) (InFromSlotInfo :type S%20GR%20Inven%20Slot%20Info%20Structure)))

(fn TryAddItemListBase
  (params (InItemInfoRefArray :type Array%20of%20BPO%20GR%20Inven%20Item%20Info%20Object%20References))
  (for _array_element InItemInfoRefArray
    (Base|TryAddItemBase _array_element)))

(fn InitWidgetsBase
  (params (InputContainerWidget :type User%20Widget%20Object%20Reference) (InWidgetSlotChunkInfoArray :type Array%20of%20S%20GR%20Widget%20Slot%20Chunk%20Info%20Structures))
  (Variables|Default|SetContainerWidget InputContainerWidget)
  (Variables|Default|SetWidgetSlotChunkInfoArray InWidgetSlotChunkInfoArray)
  (for _index (range 0 (- (Utilities|Array|Length (Variables|Default|GetWidgetSlotChunkInfoArray)) 1))
    (LocalVariables|SetLocalChunkIndex _index)
    (Utilities|FlowControl|Sequence
      (:then_0
        (for (_array_element _array_index) (.InvenSlotWidgets (Utilities|Struct|BreakS_GR_WidgetSlotChunkInfo (Utilities|Array|Get(acopy) (Variables|Default|GetWidgetSlotChunkInfoArray) (LocalVariables|GetLocalChunkIndex))))
          (Class|BPIGRSlotWidgetInterface|SetSlotID(Message) _array_element (Utilities|Struct|MakeS_GR_InvenSlotID (LocalVariables|GetLocalChunkIndex) _array_index self))))
      (:then_1
        (for (_array_element_2 _array_index_2) (.InvenItemWidgets (Utilities|Struct|BreakS_GR_WidgetSlotChunkInfo (Utilities|Array|Get(acopy) (Variables|Default|GetWidgetSlotChunkInfoArray) (LocalVariables|GetLocalChunkIndex))))
          (Class|BPIGRSlotWidgetInterface|SetSlotID(Message) _array_element_2 (Utilities|Struct|MakeS_GR_InvenSlotID (LocalVariables|GetLocalChunkIndex) _array_index_2 self))))))
  (Base|UpdateWidgetsBase))

(fn UpdateWidgetbySlotInfoBase
  (params (InSlotInfo :type S%20GR%20Inven%20Slot%20Info%20Structure) (InReCreateIconTexture :type Boolean)))

(fn TryAddStackableItemBase
  (params (InInvenItemInfoRef :type BPO%20GR%20Inven%20Item%20Info%20Object%20Reference))
  (bind (_found _returnvalue) (Default|FindItemDataFl (Variables|Default|GetOwnerInventory) InInvenItemInfoRef))
  (if _found
    (if (.AllowStacking (Utilities|Struct|BreakS_GR_ItemTableData _returnvalue))
      (bind _returnvaluearray (Base|GetAllItemsBase))
      (for _array_element _returnvaluearray
        (bind _output_get (LocalVariables|SetLocalToItemInfoRef _array_element))
        (bind _returnvalue_2 (Default|CheckSameTypeItemFl (Variables|Default|GetOwnerInventory) _output_get InInvenItemInfoRef))
        (if _returnvalue_2
          (bind _returnvalue_3 (Default|FindItemDataFl (Variables|Default|GetOwnerInventory) (LocalVariables|GetLocalToItemInfoRef)))
          (bind _output_get_2 (LocalVariables|SetLocalToItemData _returnvalue_3))
          (bind _output_get_3 (LocalVariables|SetLocalEmptyAmount (- (.MaxStack (Utilities|Struct|BreakS_GR_ItemTableData _output_get_2)) (Variables|/Game/AdvRPGInventory/Blueprints/UObjects/BPO_GR_InvenItemInfo.BPO_GR_InvenItemInfo_C|GetAmount (LocalVariables|GetLocalToItemInfoRef)))))
          (if (> _output_get_3 0)
            (bind _output_get_4 (LocalVariables|SetLocaMoveItemRemainAmount (Math|Integer|Clamp(Integer) (- (Variables|/Game/AdvRPGInventory/Blueprints/UObjects/BPO_GR_InvenItemInfo.BPO_GR_InvenItemInfo_C|GetAmount InInvenItemInfoRef) (LocalVariables|GetLocalEmptyAmount)) 0 (.MaxStack (Utilities|Struct|BreakS_GR_ItemTableData (LocalVariables|GetLocalToItemData))))))
            (if (> _output_get_4 0)
              (Variables|/Game/AdvRPGInventory/Blueprints/UObjects/BPO_GR_InvenItemInfo.BPO_GR_InvenItemInfo_C|SetAmount (LocalVariables|GetLocalToItemInfoRef) (.MaxStack (Utilities|Struct|BreakS_GR_ItemTableData (LocalVariables|GetLocalToItemData))))
              (Variables|/Game/AdvRPGInventory/Blueprints/UObjects/BPO_GR_InvenItemInfo.BPO_GR_InvenItemInfo_C|SetAmount InInvenItemInfoRef (LocalVariables|GetLocaMoveItemRemainAmount))
              (else
                (Variables|/Game/AdvRPGInventory/Blueprints/UObjects/BPO_GR_InvenItemInfo.BPO_GR_InvenItemInfo_C|SetAmount (LocalVariables|GetLocalToItemInfoRef) (+ (Variables|/Game/AdvRPGInventory/Blueprints/UObjects/BPO_GR_InvenItemInfo.BPO_GR_InvenItemInfo_C|GetAmount InInvenItemInfoRef) (Variables|/Game/AdvRPGInventory/Blueprints/UObjects/BPO_GR_InvenItemInfo.BPO_GR_InvenItemInfo_C|GetAmount (LocalVariables|GetLocalToItemInfoRef))))
                (return true))))))
      (bind _returnvalue_4 (Default|EmptyAmount InInvenItemInfoRef))
      (if (not _returnvalue_4)
        (bind _returnvalue_5 (Base|TryAddItemBase InInvenItemInfoRef))
        (return _returnvalue_5))
      (else
        (bind _returnvalue_6 (Base|TryAddItemBase InInvenItemInfoRef))
        (return _returnvalue_6)))))

(fn FindItemInfotoSwapBase
  (params (InMoveItemInfoRef :type BPO%20GR%20Inven%20Item%20Info%20Object%20Reference) (InFromSlotInfo :type S%20GR%20Inven%20Slot%20Info%20Structure) (InToSlotInfo :type S%20GR%20Inven%20Slot%20Info%20Structure))
  (return false 0))

(fn TryPlaceItemBase
  (params (InPlaceInvenItemInfoRef :type BPO%20GR%20Inven%20Item%20Info%20Object%20Reference) (InToSlotInfo :type S%20GR%20Inven%20Slot%20Info%20Structure) (InFromSlotInfo :type S%20GR%20Inven%20Slot%20Info%20Structure))
  (return false ""))

(fn TryFillStackItemBase
  (params (InFromSlotInfo :type S%20GR%20Inven%20Slot%20Info%20Structure) (InToSlotInfo :type S%20GR%20Inven%20Slot%20Info%20Structure) (InMoveItemInfoRef :type BPO%20GR%20Inven%20Item%20Info%20Object%20Reference))
  (return false 0 ""))

(fn CanFillStackItemBase
  (params (InFromSlotInfo :type S%20GR%20Inven%20Slot%20Info%20Structure) (InToSlotInfo :type S%20GR%20Inven%20Slot%20Info%20Structure) (InMoveItemInfoRef :type BPO%20GR%20Inven%20Item%20Info%20Object%20Reference))
  (return false 0 ""))

(fn CanPlaceItemBase
  (params (InMoveItemInfoRef :type BPO%20GR%20Inven%20Item%20Info%20Object%20Reference) (InFromSlotInfo :type S%20GR%20Inven%20Slot%20Info%20Structure) (InToSlotInfo :type S%20GR%20Inven%20Slot%20Info%20Structure) (InBlockSlotIndexArray :type Array%20of%20Integers) (InIgnoreItemRefArray :type Array%20of%20BPO%20GR%20Inven%20Item%20Info%20Object%20References))
  (return false))

(fn GetAreaSlotIndexArraybyItemInfoBase
  (params (InToSlotInfo :type S%20GR%20Inven%20Slot%20Info%20Structure) (InInvenItemInfoRef :type BPO%20GR%20Inven%20Item%20Info%20Object%20Reference))
  (return 0 0))

(fn TryRemoveItembyGuidBase
  (params (InGuid :type Guid%20Structure))
  (for _array_element (Variables|Default|GetSlotChunkInfoArray)
    (for _array_element_2 (Utilities|Struct|BreakS_GR_SlotChunkInfo _array_element)
      (bind _output_get (LocalVariables|SetLocalSlotInfo _array_element_2))
      (Utilities|IsValid (Utilities|Struct|BreakS_GR_InvenSlotInfo _output_get)
        (:Is%20Valid
          (if (== (Variables|/Game/AdvRPGInventory/Blueprints/UObjects/BPO_GR_InvenItemInfo.BPO_GR_InvenItemInfo_C|GetGuid (Utilities|Struct|BreakS_GR_InvenSlotInfo _output_get)) InGuid)
            (Base|ClearItemInfoBase (LocalVariables|GetLocalSlotInfo))
            (return true))))))
  (return false))

(fn GetItemInfobySlotIndexBase
  (params (InChunkIndex :type Integer) (InSlotIndex :type Integer))
  (return (Utilities|Struct|BreakS_GR_InvenSlotInfo (Base|GetSlotInfobyIndexBase InChunkIndex InSlotIndex))))

(fn UpdateWidgetbyItemInfoBase
  (params (InReCreateIconTexture :type Boolean) (InInvenItemInfoRef :type BPO%20GR%20Inven%20Item%20Info%20Object%20Reference)))

(fn GetInvenItemWidgetbyIndexBase
  (params (InChunkIndex :type Integer) (InSlotIndex :type Integer))
  (if (Utilities|Array|IsValidIndex (Variables|Default|GetWidgetSlotChunkInfoArray) InChunkIndex)
    (return (Utilities|Array|Get(acopy) (Utilities|Struct|BreakS_GR_WidgetSlotChunkInfo (Utilities|Array|Get(acopy) (Variables|Default|GetWidgetSlotChunkInfoArray) InChunkIndex)) InSlotIndex))))

(fn GetInvenSlotWidgetbyIndexBase
  (params (InChunkIndex :type Integer) (InSlotIndex :type Integer))
  (if (Utilities|Array|IsValidIndex (Variables|Default|GetWidgetSlotChunkInfoArray) InChunkIndex)
    (return (Utilities|Array|Get(acopy) (Utilities|Struct|BreakS_GR_WidgetSlotChunkInfo (Utilities|Array|Get(acopy) (Variables|Default|GetWidgetSlotChunkInfoArray) InChunkIndex)) InSlotIndex))))

(fn ResetSlotChunkInfoArrayBase
  (for _index (range 0 (- (Utilities|Array|Length (Variables|Default|GetSlotChunkInfoArray)) 1))
    (LocalVariables|SetLocalChunkIndex _index)
    (for _index_2 (range 0 (- (Utilities|Array|Length (Utilities|Struct|BreakS_GR_SlotChunkInfo (Utilities|Array|Get(acopy) (Variables|Default|GetSlotChunkInfoArray) (LocalVariables|GetLocalChunkIndex)))) 1))
      (LocalVariables|SetLocalSlotIndex _index_2)
      (Utilities|Struct|SetmembersinS_GR_InvenSlotInfo (Utilities|Array|Get(acopy) (Utilities|Struct|BreakS_GR_SlotChunkInfo (Utilities|Array|Get(acopy) (Variables|Default|GetSlotChunkInfoArray) (LocalVariables|GetLocalChunkIndex))) (LocalVariables|GetLocalSlotIndex)) (LocalVariables|GetLocalChunkIndex) (LocalVariables|GetLocalSlotIndex) 0 self "NewEnumerator3"))))

(fn GetItemInfobySlotBase
  (params (InInvenSlot :type S%20GR%20Inven%20Slot%20Info%20Structure))
  (bind (_chunkindex _slotindex) (Utilities|Struct|BreakS_GR_InvenSlotInfo InInvenSlot))
  (return (Utilities|Struct|BreakS_GR_InvenSlotInfo (Base|GetSlotInfobyIndexBase _chunkindex _slotindex))))

(fn ContainsItembyGuidBase
  (params (InCheckItemGuid :type Guid%20Structure))
  (bind _returnvaluearray (Base|GetAllItemsBase))
  (for _array_element _returnvaluearray
    (if (== (Variables|/Game/AdvRPGInventory/Blueprints/UObjects/BPO_GR_InvenItemInfo.BPO_GR_InvenItemInfo_C|GetGuid _array_element) InCheckItemGuid)
      (return true)))
  (return false))

(fn FindItembyGuidBase
  (params (InCheckItemGuid :type Guid%20Structure))
  (bind _returnvaluearray (Base|GetAllItemsBase))
  (for _array_element _returnvaluearray
    (if (== (Variables|/Game/AdvRPGInventory/Blueprints/UObjects/BPO_GR_InvenItemInfo.BPO_GR_InvenItemInfo_C|GetGuid _array_element) InCheckItemGuid)
      (return true _array_element)))
  (return false 0))

(fn FindSlotInfobyItemInfoBase
  (params (InInvenItemInfoRef :type BPO%20GR%20Inven%20Item%20Info%20Object%20Reference))
  (bind (_found _returnslotinfo) (Base|FindSlotInfobyItemGuidBase (Variables|/Game/AdvRPGInventory/Blueprints/UObjects/BPO_GR_InvenItemInfo.BPO_GR_InvenItemInfo_C|GetGuid InInvenItemInfoRef)))
  (return _found _returnslotinfo))

(fn FindSlotInfobyItemGuidBase
  (params (InItemGuid :type Guid%20Structure))
  (for _array_element (Variables|Default|GetSlotChunkInfoArray)
    (for _array_element_2 (Utilities|Struct|BreakS_GR_SlotChunkInfo _array_element)
      (Utilities|IsValid (Utilities|Struct|BreakS_GR_InvenSlotInfo _array_element_2)
        (:Is%20Valid
          (if (== (Variables|/Game/AdvRPGInventory/Blueprints/UObjects/BPO_GR_InvenItemInfo.BPO_GR_InvenItemInfo_C|GetGuid (Utilities|Struct|BreakS_GR_InvenSlotInfo _array_element_2)) InItemGuid)
            (return true _array_element_2)))))))

(fn GetAllItemsBase
  (for _array_element (Variables|Default|GetSlotChunkInfoArray)
    (for _array_element_2 (Utilities|Struct|BreakS_GR_SlotChunkInfo _array_element)
      (Utilities|IsValid (Utilities|Struct|BreakS_GR_InvenSlotInfo _array_element_2)
        (:Is%20Valid
          (Utilities|Array|AddUnique (LocalVariables|GetLocalItemInfoArray) (Utilities|Struct|BreakS_GR_InvenSlotInfo _array_element_2))))))
  (return (LocalVariables|GetLocalItemInfoArray)))

(fn ClearItemInfoBase
  (params (InSlotInfo :type S%20GR%20Inven%20Slot%20Info%20Structure))
  (bind (_chunkindex _slotindex) (Utilities|Struct|BreakS_GR_InvenSlotInfo InSlotInfo))
  (Utilities|Struct|SetmembersinS_GR_InvenSlotInfo (Utilities|Array|Get(acopy) (Utilities|Struct|BreakS_GR_SlotChunkInfo (Utilities|Array|Get(acopy) (Variables|Default|GetSlotChunkInfoArray) _chunkindex)) _slotindex) 0))

(fn SetItemInfoBase
  (params (InSlotInfo :type S%20GR%20Inven%20Slot%20Info%20Structure) (InInvenItemInfoRef :type BPO%20GR%20Inven%20Item%20Info%20Object%20Reference))
  (bind (_chunkindex _slotindex) (Utilities|Struct|BreakS_GR_InvenSlotInfo InSlotInfo))
  (Utilities|Struct|SetmembersinS_GR_InvenSlotInfo (Utilities|Array|Get(acopy) (Utilities|Struct|BreakS_GR_SlotChunkInfo (Utilities|Array|Get(acopy) (Variables|Default|GetSlotChunkInfoArray) _chunkindex)) _slotindex) InInvenItemInfoRef))

(fn RemoveAllItemsBase
  (for _array_element (Variables|Default|GetSlotChunkInfoArray)
    (for _array_element_2 (Utilities|Struct|BreakS_GR_SlotChunkInfo _array_element)
      (Utilities|IsValid (Utilities|Struct|BreakS_GR_InvenSlotInfo _array_element_2)
        (:Is%20Valid
          (Base|ClearItemInfoBase _array_element_2))))))

(fn CreateSaveItemInfoArry
  (for _array_element (Variables|Default|GetSlotChunkInfoArray)
    (for _array_element_2 (Utilities|Struct|BreakS_GR_SlotChunkInfo _array_element)
      (LocalVariables|SetLocalSlotInfo _array_element_2)
      (Utilities|IsValid (Utilities|Struct|BreakS_GR_InvenSlotInfo _array_element_2)
        (:Is%20Valid
          (bind _returnvalue (Default|CreateStruct (Utilities|Struct|BreakS_GR_InvenSlotInfo _array_element_2)))
          (bind _output_get (LocalVariables|SetLocalItemInfoS _returnvalue))
          (bind _structout (Utilities|Struct|SetmembersinS_GR_InvenItemInfo _output_get (Utilities|Struct|MakeS_GR_InvenSlotID (.ChunkIndex (Utilities|Struct|BreakS_GR_InvenSlotInfo (LocalVariables|GetLocalSlotInfo))) (.SlotIndex (Utilities|Struct|BreakS_GR_InvenSlotInfo (LocalVariables|GetLocalSlotInfo))) 0)))
          (Utilities|Array|Add (LocalVariables|GetLocalItemSaveInfoArray) (Utilities|Struct|MakeS_GR_InvenItemSaveInfo _structout -1))))))
  (return (LocalVariables|GetLocalItemSaveInfoArray)))

(fn TryAddItemInfofromSave
  (params (InItemSaveInfo :type S%20GR%20Inven%20Item%20Save%20Info%20Structure))
  (bind _inveniteminfo (Utilities|Struct|BreakS_GR_InvenItemSaveInfo InItemSaveInfo))
  (bind _slotid (Utilities|Struct|BreakS_GR_InvenItemInfo _inveniteminfo))
  (bind (_chunkindex _slotindex) (Utilities|Struct|BreakS_GR_InvenSlotID _slotid))
  (bind _returnvalue (Game|ConstructObjectfromClass "/Game/AdvRPGInventory/Blueprints/UObjects/BPO_GR_InvenItemInfo.BPO_GR_InvenItemInfo_C"))
  (bind _output_get (LocalVariables|SetLocalItemInfoRef _returnvalue))
  (Default|SetMembersfromStruct _output_get _inveniteminfo)
  (Base|SetItemInfoBase (Utilities|Struct|MakeS_GR_InvenSlotInfo _chunkindex _slotindex) (LocalVariables|GetLocalItemInfoRef))
  (return (LocalVariables|GetLocalItemInfoRef)))

(fn FindEmptySlot
  (for _array_element (Variables|Default|GetSlotChunkInfoArray)
    (for _array_element_2 (Utilities|Struct|BreakS_GR_SlotChunkInfo _array_element)
      (Utilities|IsValid (Utilities|Struct|BreakS_GR_InvenSlotInfo _array_element_2)
        (:Is%20Not%20Valid
          (return true _array_element_2))))
    (return false "")))

(fn TryAddItemListbyLootItemInfoBase
  (params (InLootItemInfoArray :type Array%20of%20S%20GR%20Loot%20Item%20Info%20Structures))
  (if (> (Utilities|Array|Length InLootItemInfoArray) 0)
    (for _array_element InLootItemInfoArray
      (bind _returnvalue (Game|ConstructObjectfromClass "/Game/AdvRPGInventory/Blueprints/UObjects/BPO_GR_InvenItemInfo.BPO_GR_InvenItemInfo_C"))
      (bind _output_get (LocalVariables|SetLocalItemInfoRef _returnvalue))
      (Default|SetMembersbyLootInfo _output_get _array_element)
      (Base|TryAddItemBase (LocalVariables|GetLocalItemInfoRef)))))