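; Inventory grid container that shows items filtered by category, backed by a hidden "All" origin grid container it constructs on init.
; UpdateCategory clears the visible slots, then refills them from the origin, either packing matching items into free slots or copying the exact layout for All.
; Placing and clearing items write back to the origin: add or remove in category views, full slot-by-slot copy in All view.
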(fn TryPlaceItemBase
  (params (InPlaceInvenItemInfoRef :type BPO%20GR%20Inven%20Item%20Info%20Object%20Reference) (InToSlotInfo :type S%20GR%20Inven%20Slot%20Info%20Structure) (InFromSlotInfo :type S%20GR%20Inven%20Slot%20Info%20Structure))
  (bind (_result _returnplaceiteminfo) (|CallParentFunction InPlaceInvenItemInfoRef InToSlotInfo InFromSlotInfo))
  (LocalVariables|SetLocalResult _result)
  (LocalVariables|SetLocalPlaceItemInfo _returnplaceiteminfo)
  (Utilities|FlowControl|Sequence
    (:then_0
      (if (LocalVariables|GetLocalResult)
        (switch Utilities|FlowControl|Switch|SwitchonE_GR_InvenItemCategoryType (Variables|Default|GetCategoryType)
          (:NewEnumerator0
            (Default|TryAddItemBase (Variables|Default|GetOriginGridContainer) InPlaceInvenItemInfoRef InFromSlotInfo :!label _label))
          (:NewEnumerator2
            (goto _label))
          (:NewEnumerator1
            (goto _label))
          (:NewEnumerator3
            (goto _label))
          (:NewEnumerator5
            (for (_array_element _array_index) (Variables|Default|GetSlotChunkInfoArray)
              (LocalVariables|SetLocalChunkIndex _array_index)
              (for (_array_element_2 _array_index_2) (Utilities|Struct|BreakS_GR_SlotChunkInfo _array_element)
                (LocalVariables|SetLocalSlotIndex _array_index_2)
                (Utilities|Struct|SetmembersinS_GR_InvenSlotInfo (Utilities|Array|Get(acopy) (Utilities|Struct|BreakS_GR_SlotChunkInfo (Utilities|Array|Get(acopy) (Variables|/Game/AdvRPGInventory/Blueprints/UObjects/BPO_GR_BaseContainer.BPO_GR_BaseContainer_C|GetSlotChunkInfoArray (Variables|Default|GetOriginGridContainer)) (LocalVariables|GetLocalChunkIndex))) (LocalVariables|GetLocalSlotIndex)) (Utilities|Struct|BreakS_GR_InvenSlotInfo _array_element_2))))))))
    (:then_1
      (return (LocalVariables|GetLocalResult) (LocalVariables|GetLocalPlaceItemInfo)))))

(fn ClearItemInfoBase
  (params (InSlotInfo :type S%20GR%20Inven%20Slot%20Info%20Structure))
  (bind (_chunkindex _slotindex) (Utilities|Struct|BreakS_GR_InvenSlotInfo InSlotInfo))
  (LocalVariables|SetLocalRemoveItemInfo (CallFunction|GetItemInfobySlotIndexBase _chunkindex _slotindex))
  (|CallParentFunction InSlotInfo)
  (switch Utilities|FlowControl|Switch|SwitchonE_GR_InvenItemCategoryType (Variables|Default|GetCategoryType)
    (:NewEnumerator0
      (bind _returnvalue (Default|TryRemoveItemBase (Variables|Default|GetOriginGridContainer) (LocalVariables|GetLocalRemoveItemInfo) :!label _label))
      (if _returnvalue
        _))
    (:NewEnumerator2
      (goto _label))
    (:NewEnumerator1
      (goto _label))
    (:NewEnumerator3
      (goto _label))
    (:NewEnumerator5
      (for (_array_element _array_index) (Variables|Default|GetSlotChunkInfoArray)
        (LocalVariables|SetLocalChunkIndex _array_index)
        (for (_array_element_2 _array_index_2) (Utilities|Struct|BreakS_GR_SlotChunkInfo _array_element)
          (LocalVariables|SetLocalSlotIndex _array_index_2)
          (Utilities|Struct|SetmembersinS_GR_InvenSlotInfo (Utilities|Array|Get(acopy) (Utilities|Struct|BreakS_GR_SlotChunkInfo (Utilities|Array|Get(acopy) (Variables|/Game/AdvRPGInventory/Blueprints/UObjects/BPO_GR_BaseContainer.BPO_GR_BaseContainer_C|GetSlotChunkInfoArray (Variables|Default|GetOriginGridContainer)) (LocalVariables|GetLocalChunkIndex))) (LocalVariables|GetLocalSlotIndex)) (Utilities|Struct|BreakS_GR_InvenSlotInfo _array_element_2)))))))

(fn InitBase
  (params (InContainerName :type Name :default "None") (InOwnerInventory :type BPO%20GR%20Inventory%20Object%20Reference) (InSlotChunkInfoArray :type Array%20of%20S%20GR%20Slot%20Chunk%20Info%20Structures))
  (|CallParentFunction InContainerName InOwnerInventory InSlotChunkInfoArray)
  (bind _returnvalue (Game|ConstructObjectfromClass "/Game/AdvRPGInventory/Blueprints/UObjects/BPO_GR_GridContainer.BPO_GR_GridContainer_C"))
  (bind _output_get (Variables|Default|SetOriginGridContainer _returnvalue))
  (CallFunction|InitBase _output_get "All" InOwnerInventory InSlotChunkInfoArray)
  (return))

(fn UpdateCategory
  (params (InItemCategoryType :type E_GR_InvenItemCategoryType%20Enum :default "NewEnumerator0"))
  (Variables|Default|SetCategoryType InItemCategoryType)
  (Utilities|FlowControl|Sequence
    (:then_0
      (for (_array_element _array_index) (Variables|Default|GetSlotChunkInfoArray)
        (LocalVariables|SetLocalChunkIndex _array_index)
        (for (_ _array_index_2) (Utilities|Struct|BreakS_GR_SlotChunkInfo _array_element)
          (LocalVariables|SetLocalSlotIndex _array_index_2)
          (Utilities|Struct|SetmembersinS_GR_InvenSlotInfo (Utilities|Array|Get(acopy) (Utilities|Struct|BreakS_GR_SlotChunkInfo (Utilities|Array|Get(acopy) (Variables|Default|GetSlotChunkInfoArray) (LocalVariables|GetLocalChunkIndex))) (LocalVariables|GetLocalSlotIndex)) 0))))
    (:then_1
      (switch Utilities|FlowControl|Switch|SwitchonE_GR_InvenItemCategoryType (Variables|Default|GetCategoryType)
        (:NewEnumerator0
          (bind _returnvaluearray (Default|GetAllItemsBase (Variables|Default|GetOriginGridContainer) :!label _label))
          (for _array_element_2 _returnvaluearray
            (bind _output_get (LocalVariables|SetLocalItemInfoRef _array_element_2))
            (bind _returnvalue (Default|FindItemDataFl (Variables|Default|GetOwnerInventory) _output_get))
            (if (Utilities|Enum|Equal(Enum) (Utilities|Struct|BreakS_GR_ItemTableData _returnvalue) (Variables|Default|GetCategoryType))
              (CallFunction|TryAddItem2 (LocalVariables|GetLocalItemInfoRef)))))
        (:NewEnumerator2
          (goto _label))
        (:NewEnumerator1
          (goto _label))
        (:NewEnumerator3
          (goto _label))
        (:NewEnumerator5
          (for (_array_element_3 _array_index_3) (Variables|/Game/AdvRPGInventory/Blueprints/UObjects/BPO_GR_BaseContainer.BPO_GR_BaseContainer_C|GetSlotChunkInfoArray (Variables|Default|GetOriginGridContainer))
            (LocalVariables|SetLocalChunkIndex _array_index_3)
            (for (_array_element_4 _array_index_4) (Utilities|Struct|BreakS_GR_SlotChunkInfo _array_element_3)
              (LocalVariables|SetLocalSlotIndex _array_index_4)
              (Utilities|Struct|SetmembersinS_GR_InvenSlotInfo (Utilities|Array|Get(acopy) (Utilities|Struct|BreakS_GR_SlotChunkInfo (Utilities|Array|Get(acopy) (Variables|Default|GetSlotChunkInfoArray) (LocalVariables|GetLocalChunkIndex))) (LocalVariables|GetLocalSlotIndex)) (Utilities|Struct|BreakS_GR_InvenSlotInfo _array_element_4)))))))
    (:then_2
      (CallFunction|UpdateWidgetsBase))))

(fn TryAddItem2
  (params (InInvenItemInfoRef :type BPO%20GR%20Inven%20Item%20Info%20Object%20Reference))
  (for (_array_element _array_index) (Variables|Default|GetSlotChunkInfoArray)
    (LocalVariables|SetLocalChunkIndex _array_index)
    (for (_array_element_2 _array_index_2) (Utilities|Struct|BreakS_GR_SlotChunkInfo _array_element)
      (LocalVariables|SetLocalSlotIndex _array_index_2)
      (Utilities|IsValid (Utilities|Struct|BreakS_GR_InvenSlotInfo _array_element_2)
        (:Is%20Not%20Valid
          (Utilities|Struct|SetmembersinS_GR_InvenSlotInfo (Utilities|Array|Get(acopy) (Utilities|Struct|BreakS_GR_SlotChunkInfo (Utilities|Array|Get(acopy) (Variables|Default|GetSlotChunkInfoArray) (LocalVariables|GetLocalChunkIndex))) (LocalVariables|GetLocalSlotIndex)) InInvenItemInfoRef)
          (return true))))))