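; Blueprint function library of shared helpers for the RPG inventory, covering items, slots and containers.
; Items resolve their data through DataTable row handles, and slot operations are forwarded to the owning container.
; Items can own inventories of containers, so recursive searches walk nested contents for containment checks and widget refreshes.
; Other helpers handle stacking, splitting and removing amounts, magazine and weapon ammo counts, grid index math and on-screen text messages.
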(fn FindItemData
  (params (InInvenItemInfoRef :type BPO%20GR%20Inven%20Item%20Info%20Object%20Reference))
  (bind _datatablehandle (Variables|/Game/AdvRPGInventory/Blueprints/UObjects/BPO_GR_InvenItemInfo.BPO_GR_InvenItemInfo_C|GetDataTableHandle InInvenItemInfoRef))
  (bind (_datatable _rowname) (Utilities|Struct|BreakDataTableRowHandle _datatablehandle))
  (Utilities|IsValid InInvenItemInfoRef
    (:Is%20Valid
      (Utilities|IsValid _datatable
        (:Is%20Valid
          (bind _returnvalue (Utilities|GetDataTableRow _datatable _rowname)
            (:then
              (return true _returnvalue))
            (:RowNotFound
              (return false ""))))))
    (:Is%20Not%20Valid
      (Development|PrintString 0))))

(fn FindItemDatabyTableRow
  (params (InDTRowHandle :type Data%20Table%20Row%20Handle%20Structure))
  (bind (_datatable _rowname) (Utilities|Struct|BreakDataTableRowHandle InDTRowHandle))
  (bind _returnvalue (Utilities|GetDataTableRow _datatable _rowname)
    (:then
      (return true _returnvalue))
    (:RowNotFound
      (return false ""))))

(fn FindItemInventoryData
  (params (InInvenItemInfoRef :type BPO%20GR%20Inven%20Item%20Info%20Object%20Reference))
  (bind _datatablehandle (Variables|/Game/AdvRPGInventory/Blueprints/UObjects/BPO_GR_InvenItemInfo.BPO_GR_InvenItemInfo_C|GetDataTableHandle InInvenItemInfoRef))
  (bind (_datatable _rowname) (Utilities|Struct|BreakDataTableRowHandle _datatablehandle))
  (Utilities|IsValid _datatable
    (:Is%20Valid
      (bind _returnvalue (Utilities|GetDataTableRow _datatable _rowname)
        (:then
          (Utilities|IsValid (.DataTable (Utilities|Struct|BreakDataTableRowHandle (.InventoryTableRow (Utilities|Struct|BreakS_GR_ItemTableData _returnvalue))))
            (:Is%20Valid
              (bind _returnvalue_2 (Utilities|GetDataTableRow (.DataTable (Utilities|Struct|BreakDataTableRowHandle (.InventoryTableRow (Utilities|Struct|BreakS_GR_ItemTableData _returnvalue)))) (.RowName (Utilities|Struct|BreakDataTableRowHandle (.InventoryTableRow (Utilities|Struct|BreakS_GR_ItemTableData _returnvalue)))))
                (:then
                  (return true _returnvalue_2))
                (:RowNotFound
                  _)))
            (:Is%20Not%20Valid
              _))
          (return false ""))))))

(fn FindItemInfobySlot
  (params (InInvenSlotInfo :type S%20GR%20Inven%20Slot%20Info%20Structure))
  (bind _inveniteminforef (Utilities|Struct|BreakS_GR_InvenSlotInfo InInvenSlotInfo))
  (Utilities|FlowControl|Sequence
    (:then_0
      (Utilities|IsValid _inveniteminforef
        (:Is%20Valid
          (return true _inveniteminforef))))
    (:then_1
      (return false 0))))

(fn IsIntersectDeprecated
  (params (x1 :type Integer) (y1 :type Integer) (w1 :type Integer) (h1 :type Integer) (x2 :type Integer) (y2 :type Integer) (w2 :type Integer) (h2 :type Integer))
  (return (Math|Boolean|ANDBoolean (>= (+ x1 w1) x2) (<= x1 (+ x2 w2)) (>= (+ y1 h1) y2) (<= y1 (+ y2 h2)))))

(fn FindItemInfobySlotID
  (params (InSlotID :type S%20GR%20Inven%20Slot%20ID%20Structure))
  (bind _returnslotinfo (CallFunction|GetSlotInfobySlotID InSlotID))
  (bind (_found _returnvalueref) (CallFunction|FindItemInfobySlot _returnslotinfo))
  (return _found _returnvalueref))

(fn SetItemInfotoSlot
  (params (InToInvenSlotInfo :type S%20GR%20Inven%20Slot%20Info%20Structure) (InInvenItemInfoRef :type BPO%20GR%20Inven%20Item%20Info%20Object%20Reference))
  (Default|SetItemInfoBase (Utilities|Struct|BreakS_GR_InvenSlotInfo InToInvenSlotInfo) InToInvenSlotInfo InInvenItemInfoRef))

(fn SetItemContainerOwnerActor
  (params (InInvenItemInfoRef :type BPO%20GR%20Inven%20Item%20Info%20Object%20Reference) (InOwnerActor :type Actor%20Object%20Reference))
  (bind _inventoryref (Variables|/Game/AdvRPGInventory/Blueprints/UObjects/BPO_GR_InvenItemInfo.BPO_GR_InvenItemInfo_C|GetInventoryRef InInvenItemInfoRef))
  (Utilities|IsValid _inventoryref
    (:Is%20Valid
      (for _array_element (Variables|/Game/AdvRPGInventory/Blueprints/UObjects/BPO_GR_Inventory.BPO_GR_Inventory_C|GetContainerArray _inventoryref)
        (Variables|/Game/AdvRPGInventory/Blueprints/UObjects/BPO_GR_BaseContainer.BPO_GR_BaseContainer_C|SetOwnerActor _array_element InOwnerActor)))))

(fn SetItemAmountbySlot
  (params (InInvenSlotInfo :type S%20GR%20Inven%20Slot%20Info%20Structure) (InAmount :type Integer))
  (bind _inveniteminforef (Utilities|Struct|BreakS_GR_InvenSlotInfo InInvenSlotInfo))
  (Utilities|IsValid _inveniteminforef
    (:Is%20Valid
      (Variables|/Game/AdvRPGInventory/Blueprints/UObjects/BPO_GR_InvenItemInfo.BPO_GR_InvenItemInfo_C|SetAmount _inveniteminforef InAmount))))

(fn HasContainer
  (params (InInvenItemInfoRef :type BPO%20GR%20Inven%20Item%20Info%20Object%20Reference) (InContainer :type BPO%20GR%20Base%20Container%20Object%20Reference))
  (bind _inventoryref (Variables|/Game/AdvRPGInventory/Blueprints/UObjects/BPO_GR_InvenItemInfo.BPO_GR_InvenItemInfo_C|GetInventoryRef InInvenItemInfoRef))
  (Utilities|IsValid _inventoryref
    (:Is%20Valid
      (return (Utilities|Array|ContainsItem (Variables|/Game/AdvRPGInventory/Blueprints/UObjects/BPO_GR_Inventory.BPO_GR_Inventory_C|GetContainerArray _inventoryref) InContainer)))))

(fn HasSlot
  (params (InInvenItemInfoRef :type BPO%20GR%20Inven%20Item%20Info%20Object%20Reference) (InCheckSlotInfo :type S%20GR%20Inven%20Slot%20Info%20Structure))
  (for _array_element (Variables|/Game/AdvRPGInventory/Blueprints/UObjects/BPO_GR_Inventory.BPO_GR_Inventory_C|GetContainerArray (Variables|/Game/AdvRPGInventory/Blueprints/UObjects/BPO_GR_InvenItemInfo.BPO_GR_InvenItemInfo_C|GetInventoryRef InInvenItemInfoRef))
    (if (== _array_element (Utilities|Struct|BreakS_GR_InvenSlotInfo InCheckSlotInfo))
      (return true)))
  (return false))

(fn GetContainerWeight
  (params (InContainerComp :type Actor%20Component%20Object%20Reference))
  (Utilities|FlowControl|Sequence))

(fn GetLastUpdatedSlotInfobySlotInfo
  (params (InSlotInfo :type S%20GR%20Inven%20Slot%20Info%20Structure))
  (bind (_chunkindex _slotindex _containerref) (Utilities|Struct|BreakS_GR_InvenSlotInfo InSlotInfo))
  (return (Default|GetSlotInfobyIndexBase _containerref _chunkindex _slotindex)))

(fn GetAllChildContainer
  (params (InInvenItemInfoRef :type BPO%20GR%20Inven%20Item%20Info%20Object%20Reference))
  (bind _inventoryref (Variables|/Game/AdvRPGInventory/Blueprints/UObjects/BPO_GR_InvenItemInfo.BPO_GR_InvenItemInfo_C|GetInventoryRef InInvenItemInfoRef))
  (Utilities|FlowControl|Sequence
    (:then_0
      (Utilities|IsValid _inventoryref
        (:Is%20Valid
          (Utilities|Array|AppendArray (LocalVariables|GetLocalReturnContainerArray) (Variables|/Game/AdvRPGInventory/Blueprints/UObjects/BPO_GR_Inventory.BPO_GR_Inventory_C|GetContainerArray _inventoryref))
          (for _array_element (Variables|/Game/AdvRPGInventory/Blueprints/UObjects/BPO_GR_Inventory.BPO_GR_Inventory_C|GetContainerArray (Variables|/Game/AdvRPGInventory/Blueprints/UObjects/BPO_GR_InvenItemInfo.BPO_GR_InvenItemInfo_C|GetInventoryRef InInvenItemInfoRef))
            (bind _returnvaluearray (Default|GetAllItemsBase _array_element))
            (for _array_element_2 _returnvaluearray
              (bind _returncontainerarray (CallFunction|GetAllChildContainer _array_element_2))
              (Utilities|Array|AppendArray (LocalVariables|GetLocalReturnContainerArray) _returncontainerarray))))))
    (:then_1
      (return (LocalVariables|GetLocalReturnContainerArray)))))

(fn ContainsSlotinItemRecursive
  (params (InContainerItemInfoRef :type BPO%20GR%20Inven%20Item%20Info%20Object%20Reference) (InCheckSlotInfo :type S%20GR%20Inven%20Slot%20Info%20Structure))
  (bind _returncontainerarray (CallFunction|GetAllChildContainer InContainerItemInfoRef))
  (return (Utilities|Array|ContainsItem _returncontainerarray (.ContainerRef (Utilities|Struct|BreakS_GR_InvenSlotInfo InCheckSlotInfo)))))

(fn ContainsIteminItemRecursive
  (params (InContainerItemInfoRef :type BPO%20GR%20Inven%20Item%20Info%20Object%20Reference) (InCheckItemInfoRef :type BPO%20GR%20Inven%20Item%20Info%20Object%20Reference))
  (Utilities|FlowControl|Sequence
    (:then_0
      (for _array_element (Variables|/Game/AdvRPGInventory/Blueprints/UObjects/BPO_GR_Inventory.BPO_GR_Inventory_C|GetContainerArray (Variables|/Game/AdvRPGInventory/Blueprints/UObjects/BPO_GR_InvenItemInfo.BPO_GR_InvenItemInfo_C|GetInventoryRef InContainerItemInfoRef))
        (if (Default|ContainsItemBase _array_element InCheckItemInfoRef)
          (return true))))
    (:then_1
      (for _array_element_2 (Variables|/Game/AdvRPGInventory/Blueprints/UObjects/BPO_GR_Inventory.BPO_GR_Inventory_C|GetContainerArray (Variables|/Game/AdvRPGInventory/Blueprints/UObjects/BPO_GR_InvenItemInfo.BPO_GR_InvenItemInfo_C|GetInventoryRef InContainerItemInfoRef))
        (bind _returnvaluearray (Default|GetAllItemsBase _array_element_2))
        (for _array_element_3 _returnvaluearray
          (if (CallFunction|ContainsIteminItemRecursive _array_element_3 InCheckItemInfoRef)
            (return true)))))))

(fn ContainsIteminItem
  (params (InContainerItemInfoRef :type BPO%20GR%20Inven%20Item%20Info%20Object%20Reference) (InCheckItemInfoRef :type BPO%20GR%20Inven%20Item%20Info%20Object%20Reference))
  (for _array_element (Variables|/Game/AdvRPGInventory/Blueprints/UObjects/BPO_GR_Inventory.BPO_GR_Inventory_C|GetContainerArray (Variables|/Game/AdvRPGInventory/Blueprints/UObjects/BPO_GR_InvenItemInfo.BPO_GR_InvenItemInfo_C|GetInventoryRef InContainerItemInfoRef))
    (if (Default|ContainsItemBase _array_element InCheckItemInfoRef)
      (return true))))

(fn GetMagItemAmmoCount
  (params (InMagItemInfoRef :type BPO%20GR%20Inven%20Item%20Info%20Object%20Reference))
  (Utilities|FlowControl|Sequence
    (:then_0
      (bind (_found _returnvalue) (CallFunction|FindItemData InMagItemInfoRef))
      (if _found
        (bind _output_get (LocalVariables|SetLocalMagItemData _returnvalue))
        (if (Utilities|Enum|Equal(Enum) (.AttachmentType (Utilities|Struct|BreakS_GR_ItemTableData _output_get)) "NewEnumerator5")
          (bind _returnvalue_2 (Default|GetGridContainerExe (Variables|/Game/AdvRPGInventory/Blueprints/UObjects/BPO_GR_InvenItemInfo.BPO_GR_InvenItemInfo_C|GetInventoryRef InMagItemInfoRef)))
          (Utilities|IsValid _returnvalue_2
            (:Is%20Valid
              (bind _returnvaluearray (Default|GetAllItemsBase _returnvalue_2))
              (if (Utilities|Array|IsEmpty _returnvaluearray)
                (return true 0 0)
                (else
                  (bind _output_get_2 (LocalVariables|SetLocalAmmoItemInfoRef (Utilities|Array|Get(acopy) _returnvaluearray)))
                  (return true (Variables|/Game/AdvRPGInventory/Blueprints/UObjects/BPO_GR_InvenItemInfo.BPO_GR_InvenItemInfo_C|GetAmount _output_get_2) 0))))))))
    (:then_1
      (return false 0 0))))

(fn GetWeaponItemAmmoCount
  (params (InWeaponItemInfoRef :type BPO%20GR%20Inven%20Item%20Info%20Object%20Reference))
  (bind _inventoryref (Variables|/Game/AdvRPGInventory/Blueprints/UObjects/BPO_GR_InvenItemInfo.BPO_GR_InvenItemInfo_C|GetInventoryRef InWeaponItemInfoRef))
  (Utilities|FlowControl|Sequence
    (:then_0
      (bind (_found _returnvalue) (CallFunction|FindItemData InWeaponItemInfoRef))
      (if _found
        (LocalVariables|SetLocalWeaponItemData _returnvalue)
        (Utilities|IsValid _inventoryref
          (:Is%20Valid
            (bind _returnvalue_2 (Default|GetAttachmentContainerExe _inventoryref))
            (Utilities|IsValid _returnvalue_2
              (:Is%20Valid
                (bind (_returnvalue_3 _ammo _maxammo) (CallFunction|GetMagItemAmmoCount 0 _returnvalue_2))
                (return _returnvalue_3 _ammo _maxammo)))))))
    (:then_1
      (return false 0 0))))

(fn UpdateWidgetAllChildContainer
  (params (InInvenItemInfoRef :type BPO%20GR%20Inven%20Item%20Info%20Object%20Reference) (InIgnoreContainerArray :type Array%20of%20BPO%20GR%20Base%20Container%20Object%20References))
  (bind _returncontainerarray (CallFunction|GetAllChildContainer InInvenItemInfoRef))
  (for _array_element _returncontainerarray
    (if (not (Utilities|Array|ContainsItem InIgnoreContainerArray _array_element))
      (Default|UpdateWidgetsBase _array_element))))

(fn ContainsContainerinItemRecursive
  (params (InContainerItemInfoRef :type BPO%20GR%20Inven%20Item%20Info%20Object%20Reference) (InCheckContainer :type BPO%20GR%20Base%20Container%20Object%20Reference))
  (bind _returncontainerarray (CallFunction|GetAllChildContainer InContainerItemInfoRef))
  (return (Utilities|Array|ContainsItem _returncontainerarray InCheckContainer)))

(fn DoesThisItemHaveAContainer
  (params (InInvenItemInfoRef :type BPO%20GR%20Inven%20Item%20Info%20Object%20Reference))
  (return (Utilities|Array|IsNotEmpty (Variables|/Game/AdvRPGInventory/Blueprints/UObjects/BPO_GR_Inventory.BPO_GR_Inventory_C|GetContainerArray (Variables|/Game/AdvRPGInventory/Blueprints/UObjects/BPO_GR_InvenItemInfo.BPO_GR_InvenItemInfo_C|GetInventoryRef InInvenItemInfoRef)))))

(fn UpdateWidgetInvenItemInfo
  (params (InInvenItemInfoRef :type BPO%20GR%20Inven%20Item%20Info%20Object%20Reference))
  (for _array_element (Variables|/Game/AdvRPGInventory/Blueprints/UObjects/BPO_GR_Inventory.BPO_GR_Inventory_C|GetContainerArray (Variables|/Game/AdvRPGInventory/Blueprints/UObjects/BPO_GR_InvenItemInfo.BPO_GR_InvenItemInfo_C|GetInventoryRef InInvenItemInfoRef))
    (Default|UpdateWidgetsBase _array_element)))

(fn GetSlotInfobySlotID
  (params (InSlotID :type S%20GR%20Inven%20Slot%20ID%20Structure))
  (bind (_chunkindex _slotindex _containerref) (Utilities|Struct|BreakS_GR_InvenSlotID InSlotID))
  (return (Default|GetSlotInfobyIndexBase _containerref _chunkindex _slotindex)))

(fn UpdateWidgetbySlotInfo
  (params (InSlotInfo :type S%20GR%20Inven%20Slot%20Info%20Structure) (InReCreateIconTexture :type Boolean))
  (Default|UpdateWidgetbySlotInfoBase (Utilities|Struct|BreakS_GR_InvenSlotInfo InSlotInfo) InSlotInfo InReCreateIconTexture))

(fn FindContainerbyName
  (params (InItemInfoRef :type BPO%20GR%20Inven%20Item%20Info%20Object%20Reference%20%28by%20ref%29) (InContainerName :type Name))
  (for _array_element (Variables|/Game/AdvRPGInventory/Blueprints/UObjects/BPO_GR_Inventory.BPO_GR_Inventory_C|GetContainerArray (Variables|/Game/AdvRPGInventory/Blueprints/UObjects/BPO_GR_InvenItemInfo.BPO_GR_InvenItemInfo_C|GetInventoryRef InItemInfoRef))
    (if (== (Variables|/Game/AdvRPGInventory/Blueprints/UObjects/BPO_GR_BaseContainer.BPO_GR_BaseContainer_C|GetContainerName _array_element) InContainerName)
      (return true _array_element))))

(fn GetItemInventoryWidget
  (params (InItemInfoRef :type BPO%20GR%20Inven%20Item%20Info%20Object%20Reference))
  (bind _inventoryref (Variables|/Game/AdvRPGInventory/Blueprints/UObjects/BPO_GR_InvenItemInfo.BPO_GR_InvenItemInfo_C|GetInventoryRef InItemInfoRef))
  (Utilities|IsValid _inventoryref
    (:Is%20Valid
      (return (Variables|/Game/AdvRPGInventory/Blueprints/UObjects/BPO_GR_Inventory.BPO_GR_Inventory_C|GetInventoryWidget _inventoryref)))))

(fn GetSlotXY
  (params (InIndex :type Integer) (InColumns :type Integer))
  (return (Math|Integer|%(Integer) InIndex InColumns) (/ InIndex InColumns)))

(fn GetSlotIndex
  (params (InX :type Integer) (InY :type Integer) (InColumns :type Integer))
  (return (+ (* InY InColumns) InX)))

(fn SplitItemInfo
  (params (InInvenItemInfoRef :type BPO%20GR%20Inven%20Item%20Info%20Object%20Reference) (InFromSlotInfo :type S%20GR%20Inven%20Slot%20Info%20Structure) (InSplitAmount :type Integer))
  (bind _output_get (LocalVariables|SetLocalSplitCount__A (- (Variables|/Game/AdvRPGInventory/Blueprints/UObjects/BPO_GR_InvenItemInfo.BPO_GR_InvenItemInfo_C|GetAmount InInvenItemInfoRef) InSplitAmount)))
  (if (> _output_get 0)
    (Variables|/Game/AdvRPGInventory/Blueprints/UObjects/BPO_GR_InvenItemInfo.BPO_GR_InvenItemInfo_C|SetAmount InInvenItemInfoRef (LocalVariables|GetLocalSplitCount__A))
    (else
      (Default|ClearItemInfoBase (Utilities|Struct|BreakS_GR_InvenSlotInfo InFromSlotInfo) InFromSlotInfo)))
  (bind _returnvalue (Default|Clone InInvenItemInfoRef))
  (bind _output_get_2 (LocalVariables|SetLocalSplitItemInfoRef _returnvalue))
  (Variables|/Game/AdvRPGInventory/Blueprints/UObjects/BPO_GR_InvenItemInfo.BPO_GR_InvenItemInfo_C|SetAmount _output_get_2 InSplitAmount)
  (return (LocalVariables|GetLocalSplitItemInfoRef)))

(fn CheckSameTypeItem
  (params (InItemInfoA :type BPO%20GR%20Inven%20Item%20Info%20Object%20Reference) (InItemInfoB :type BPO%20GR%20Inven%20Item%20Info%20Object%20Reference))
  (bind _datatablehandle (Variables|/Game/AdvRPGInventory/Blueprints/UObjects/BPO_GR_InvenItemInfo.BPO_GR_InvenItemInfo_C|GetDataTableHandle InItemInfoA))
  (bind _datatablehandle_2 (Variables|/Game/AdvRPGInventory/Blueprints/UObjects/BPO_GR_InvenItemInfo.BPO_GR_InvenItemInfo_C|GetDataTableHandle InItemInfoB))
  (bind (_datatable _rowname) (Utilities|Struct|BreakDataTableRowHandle _datatablehandle))
  (bind (_datatable_2 _rowname_2) (Utilities|Struct|BreakDataTableRowHandle _datatablehandle_2))
  (return (and (== _datatable _datatable_2) (== _rowname _rowname_2))))

(fn RemoveItemInfoAmount
  (params (InInvenItemInfoRef :type BPO%20GR%20Inven%20Item%20Info%20Object%20Reference) (InFromSlotInfo :type S%20GR%20Inven%20Slot%20Info%20Structure) (InRemoveAmount :type Integer))
  (bind _output_get (LocalVariables|SetLocalSplitCount__A (- (Variables|/Game/AdvRPGInventory/Blueprints/UObjects/BPO_GR_InvenItemInfo.BPO_GR_InvenItemInfo_C|GetAmount InInvenItemInfoRef) InRemoveAmount)))
  (if (> _output_get 0)
    (Variables|/Game/AdvRPGInventory/Blueprints/UObjects/BPO_GR_InvenItemInfo.BPO_GR_InvenItemInfo_C|SetAmount InInvenItemInfoRef (LocalVariables|GetLocalSplitCount__A))
    (else
      (Default|ClearItemInfoBase (Utilities|Struct|BreakS_GR_InvenSlotInfo InFromSlotInfo) InFromSlotInfo)))
  (return))

(fn CreateTextMessage
  (params (InMessageText :type Text))
  (bind _returnvalue (UserInterface|CreateWidget "/Game/AdvRPGInventory/Blueprints/Widgets/Widget_RPG_TextMessage.Widget_RPG_TextMessage_C" 0 InMessageText))
  (UserInterface|Viewport|AddtoViewport _returnvalue 0))

(fn CanStacktoItem
  (params (InItemA :type BPO%20GR%20Inven%20Item%20Info%20Object%20Reference) (InItemB :type BPO%20GR%20Inven%20Item%20Info%20Object%20Reference))
  (Utilities|FlowControl|Sequence
    (:then_0
      (bind _returnvalue (CallFunction|CheckSameTypeItem InItemA InItemB))
      (if _returnvalue
        (bind (_found _returnvalue_2) (CallFunction|FindItemData InItemB))
        (if _found
          (bind _output_get (LocalVariables|SetLocalItemDataB _returnvalue_2))
          (if (and (.AllowStacking (Utilities|Struct|BreakS_GR_ItemTableData _output_get)) (< (Variables|/Game/AdvRPGInventory/Blueprints/UObjects/BPO_GR_InvenItemInfo.BPO_GR_InvenItemInfo_C|GetAmount InItemB) (.MaxStack (Utilities|Struct|BreakS_GR_ItemTableData _output_get))))
            (return true)))))
    (:then_1
      (return false))))